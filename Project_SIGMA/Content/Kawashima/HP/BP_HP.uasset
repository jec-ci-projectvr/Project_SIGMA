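; BP_HP is an HP bar actor that shows its fill through the "percent" material parameter on a Plane.
; BeginPlay zeroes the bar and binds AddHP to the HPChange dispatcher on the player's BP_Sphere.
; AddHP is meant to add 0.1 per event, but is marked broken.
; It reads the parameter's custom primitive data index instead of its current value.
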(event Custom|AddHP
  (bind _plane (Variables|Default|GetPlane))
  ;[1 1 1] ＨＰバー加算イベント
  (Development|PrintString "add")
  (Rendering|Material|SetScalarParameterValueonMaterials _plane "percent" (+ (Math|Conversions|ToFloat(Integer) (Class|PrimitiveComponent|GetCustomPrimitiveDataIndexforScalarParameter _plane "percent")) 0.1)))

(event EventBeginPlay
  ;[1 1 1] HPバー値初期設定
  (Rendering|Material|SetScalarParameterValueonMaterials (Variables|Default|GetPlane) "percent" 0.0)
  ;[1 1 1] イベントディスパッチャーにイベントを登録
  (bind _asbp_sphere (Utilities|Casting|CastToBP_Sphere (Game|GetPlayerCharacter 0)))
  (EventDispatchers|BindEventtoHPChange _asbp_sphere (delegate Custom|AddHP)))

(event Collision|EventActorBeginOverlap
  (params (OtherActor :type Actor%20Object%20Reference)))

(event EventTick
  (params (DeltaSeconds :type Float%20%28single-precision%29)))

(fn ConstructionScript)