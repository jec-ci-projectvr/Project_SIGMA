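; SphereBP is a player-controlled pawn that looks, moves and fires projectiles from left and right shoot points.
; Mouse axes drive controller yaw and pitch, while movement input follows the control rotation, with sensitivity and power variables set at BeginPlay.
; Each fire input spawns a ShotBP at its shoot point and passes that point's world forward vector, scaled by ShotPow, to SetVelocityInLocalSpace.
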(event EventBeginPlay
  (Variables|Default|SetLookSens 1.0)
  (Variables|Default|SetMovePow 5.0)
  (Variables|Default|SetShotPow 3e+03))

(event Collision|EventActorBeginOverlap
  (params (OtherActor :type Actor%20Object%20Reference)))

(event EventTick
  (params (DeltaSeconds :type Float%20%28single-precision%29)))

(event Input|ActionEvents|InputActionFireLeft
  (params (Key :type Key%20Structure :default "None"))
  (bind _shootleft (Variables|Default|GetshootLeft))
  (:Pressed
    (bind _returnvalue (Game|SpawnActorfromClass "/Game/Kawashima/ShotBP.ShotBP_C" (Transformation|GetWorldTransform _shootleft) "Undefined" "MultiplyWithRoot" 0 0))
    (Game|Components|ProjectileMovement|SetVelocityinLocalSpace (Variables|/Game/Kawashima/ShotBP.ShotBP_C|GetProjectileMovement _returnvalue) (* (Math|Vector|GetForwardVector (Transformation|GetWorldRotation _shootleft)) (Variables|Default|GetShotPow)))))

(event Input|ActionEvents|InputActionFireRight
  (params (Key :type Key%20Structure :default "None"))
  (bind _shootright (Variables|Default|GetshootRight))
  (:Pressed
    (bind _returnvalue (Game|SpawnActorfromClass "/Game/Kawashima/ShotBP.ShotBP_C" (Transformation|GetWorldTransform _shootright) "Undefined" "MultiplyWithRoot" 0 0))
    (Game|Components|ProjectileMovement|SetVelocityinLocalSpace (Variables|/Game/Kawashima/ShotBP.ShotBP_C|GetProjectileMovement _returnvalue) (* (Math|Vector|GetForwardVector (Transformation|GetWorldRotation _shootright)) (Variables|Default|GetShotPow)))))

(event Input|AxisEvents|InputAxisTurnRight/LeftMouse
  (params (AxisValue :type Float%20%28single-precision%29))
  (Pawn|Input|AddControllerYawInput (* AxisValue (Variables|Default|GetLookSens))))

(event Input|AxisEvents|InputAxisLookUp/DownMouse
  (params (AxisValue :type Float%20%28single-precision%29))
  (Pawn|Input|AddControllerPitchInput (* AxisValue (Variables|Default|GetLookSens))))

(event Input|AxisEvents|InputAxisMoveFor/Backward
  (params (AxisValue :type Float%20%28single-precision%29))
  (Pawn|Input|AddMovementInput (Math|Vector|GetForwardVector (Pawn|GetControlRotation :!class /Script/Engine.Pawn)) (* AxisValue (Variables|Default|GetMovePow)) false))

(event Input|AxisEvents|InputAxisMoveRight/Left
  (params (AxisValue :type Float%20%28single-precision%29))
  (Pawn|Input|AddMovementInput (Math|Vector|GetRightVector (Pawn|GetControlRotation :!class /Script/Engine.Pawn)) (* AxisValue (Variables|Default|GetMovePow)) false))

(fn ConstructionScript)