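; BP_TitlePawn is a pawn, apparently for the title screen, that handles looking around and clicking widgets.
; Mouse axes drive controller pitch and yaw, and horizontal input also rotates the spring arm locally in scaled yaw.
; Left and right fire actions each press and release a left-mouse pointer key on their own widget interaction component, so either side can operate UI.
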(event Input|ActionEvents|InputActionFireLeft
  (params (Key :type Key%20Structure :default "None"))
  (bind _widgetinteraction_l (Variables|Default|GetWidgetInteraction_L))
  (:Pressed
    (Class|WidgetInteractionComponent|PressPointerKey _widgetinteraction_l "LeftMouseButton"))
  (:Released
    (Class|WidgetInteractionComponent|ReleasePointerKey _widgetinteraction_l "LeftMouseButton")))

(event Input|ActionEvents|InputActionFireRight
  (params (Key :type Key%20Structure :default "None"))
  (bind _widgetinteraction_r (Variables|Default|GetWidgetInteraction_R))
  (:Pressed
    (Class|WidgetInteractionComponent|PressPointerKey _widgetinteraction_r "LeftMouseButton"))
  (:Released
    (Class|WidgetInteractionComponent|ReleasePointerKey _widgetinteraction_r "LeftMouseButton")))

(event Input|AxisEvents|InputAxisTurnRight/LeftMouse
  (params (AxisValue :type Float%20%28single-precision%29))
  (Pawn|Input|AddControllerYawInput AxisValue)
  (Transformation|AddLocalRotation (Variables|Default|GetSpringArm) (Math|Rotator|MakeRotator 0.0 0.0 (* AxisValue 2.5)) false false))

(event Input|AxisEvents|InputAxisLookUp/DownMouse
  (params (AxisValue :type Float%20%28single-precision%29))
  (Pawn|Input|AddControllerPitchInput AxisValue))

(fn ConstructionScript)