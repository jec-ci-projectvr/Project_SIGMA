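; VR player Blueprint that acts as a stationary-view operator, spawning and driving a BP_SphereTank remotely.
; On BeginPlay it sets stats and HMD tracking, initializes the tank with speed, sensitivity and barrier skill, then possesses it while keeping the view target on itself.
; The tank's capture component gets its render target only when locally controlled, as a bug workaround.
; Tick feeds placeholder test values to the 3D timer and table battle gauge.
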(event Custom|Player_Dead
  ;[1 0 0] 死亡時イベント
  (Development|PrintString "アナタは死にました"))

(event EventBeginPlay
  ;[1 1 1] 変数初期化
  (CallFunction|InitVariables 1e+01 5.0)
  ;[1 1 1] カメラ初期化
  (CallFunction|InitCamera)
  ;[1 1 1] Text3D初期化
  (CallFunction|InitTimeText3D)
  ;[1 1 1] 乗り物生成・初期化
  (CallFunction|InitTank (Variables|Default|GetSpawnPoint))
  ;[0.15 0.15 1 0.6] 操作対象切り替え
  (CallFunction|SetPController))

(event EventTick
  (params (DeltaSeconds :type Float%20%28single-precision%29))
  ;[0 0 1] テスト用タイマー処理
  (CallFunction|TestTimeCountUp DeltaSeconds)
  ;[0 1 1] テスト用戦況ゲージ処理(TestBattleCountUpは後に消去)
  (bind _returnvalue (CallFunction|TestBattleCountUp))
  (Rendering|Material|SetScalarParameterValueonMaterials (Variables|Default|GetMesh_Table) "Value" _returnvalue))

(fn ConstructionScript)

(fn InitVariables
  (params (HP :type Float%20%28double-precision%29) (Speed :type Float%20%28double-precision%29))
  (bind _output_get (Variables|Default|SetHP_Max HP))
  (Variables|Default|SetHP_Now _output_get)
  (Variables|Default|SetMove_Speed Speed)
  (Variables|Default|SetLook_Sens 1.0))

(fn InitCamera
  (Class|HeadMountedDisplayFunctionLibrary|SetTrackingOrigin "Eye")
  (Transformation|SetRelativeLocation (Variables|Default|GetCamera) (Math|Vector|MakeVector 0.0 0.0 2e+01) false false)
  (Class|HeadMountedDisplayFunctionLibrary|ResetOrientationandPosition 0.0 "OrientationAndPosition"))

(fn InitTank
  (params (SpawnPoint :type Transform))
  (bind _returnvalue (Game|SpawnActorfromClass "/Game/Kawashima/BP/BP_SphereTank.BP_SphereTank_C" SpawnPoint "Undefined" "MultiplyWithRoot" 0 0))
  (bind _output_get (Variables|Default|SetRef_Tank _returnvalue))
  (Variables|/Game/Kawashima/BP/BP_SphereTank.BP_SphereTank_C|SetRef_Player _output_get self)
  (Default|InitValiables _output_get (Variables|Default|GetMove_Speed) (Variables|Default|GetLook_Sens))
  (CallFunction|InitCapture _output_get)
  (Variables|/Game/Kawashima/BP/BP_SphereTank.BP_SphereTank_C|SetSkill _output_get (Variables|Default|GetBP_Skill_Barrier)))

(fn InitCapture
  (params (Tank :type BP%20Sphere%20Tank%20Object%20Reference))
  (if (Pawn|IsLocallyControlled)
    (Variables|/Script/Engine.SceneCaptureComponent2D|SetTextureTarget (Variables|/Game/Kawashima/BP/BP_SphereTank.BP_SphereTank_C|GetMain Tank) "/Game/Kawashima/Render_Main.Render_Main") ; メッシュのデフォルト値は空にしておくこと
  ))

(fn SetPController
  (bind _returnvalue (Game|GetPlayerController 0))
  (Pawn|Possess _returnvalue (Variables|Default|GetRef_Tank))
  (Game|Player|SetViewTargetwithBlend _returnvalue self 0.0 "VTBlend_Linear" 0.0 false))

(fn SetHPMaterial
  (Rendering|Material|SetScalarParameterValueonMaterials (Variables|Default|GetMesh_HP) "Value" (/ (Variables|Default|GetHP_Now) (Variables|Default|GetHP_Max))))

(fn InitTimeText3D
  (bind _asbp_time_text_3d (Utilities|Casting|CastToBP_TimeText3D (Variables|/Script/Engine.ChildActorComponent|GetChildActor (Variables|Default|GetBP_TimeText3D))))
  (Variables|Default|SetRef_TimeText3D _asbp_time_text_3d))

(fn TestTimeCountUp
  (params (A :type Float%20%28double-precision%29))
  (bind _output_get (Variables|Default|SetTestDelta (+ A (Variables|Default|GetTestDelta))))
  (if (>= _output_get 1.0)
    (Variables|Default|SetTestDelta (- (Variables|Default|GetTestDelta) 1.0))
    (bind _output_get_2 (Variables|Default|SetTestTime (+ (Variables|Default|GetTestTime) 1)))
    (Default|SetTime (Variables|Default|GetRef_TimeText3D) _output_get_2) ; 秒での経過時間ないし残り時間を渡す
  ))

(fn TestBattleCountUp
  (return (+ (* (Math|Trig|Sin(Radians) (+ (Variables|Default|GetTestDelta) (Variables|Default|GetTestTime))) 5e+01) 5e+01)))