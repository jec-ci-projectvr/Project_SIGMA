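; Blueprint debug library of helper functions that show values on screen or in the log through Print String.
; Typed variants convert strings, bools, ints, floats, vectors and transforms, or a transform's location, rotation or scale, to text.
; Append variants prefix a caller-supplied label.
; DebugLogActorInfo concatenates an actor's name, rotation and scale with the world origin location, not the actor's location, without separators.
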(fn DebugLog
  (params (Str :type String))
  (Development|PrintString 0 Str))

(fn DebugLogBool
  (params (Bool :type Boolean))
  (Development|PrintString 0 (Utilities|String|ToString(Boolean) Bool)))

(fn DebugLogInt
  (params (Int :type Integer))
  (Development|PrintString 0 (Utilities|String|ToString(Integer) Int)))

(fn DebugLogFloat
  (params (Float :type Float%20%28double-precision%29))
  (Development|PrintString 0 (Utilities|String|ToString(Float) Float)))

(fn DebugLogVector
  (params (Vec :type Vector))
  (Development|PrintString 0 (Utilities|String|ToString(Vector) Vec)))

(fn DebugLogTransform
  (params (Transform :type Transform))
  (Development|PrintString 0 (Utilities|String|ToString(Transform) Transform)))

(fn DebugLogLocation
  (params (Transform :type Transform))
  (Development|PrintString 0 (Utilities|String|ToString(Vector) (.Location (Math|Transform|BreakTransform Transform)))))

(fn DebugLogRotation
  (params (Transform :type Transform) (__WorldContext :type Object%20Object%20Reference))
  (Development|PrintString 0 (Utilities|String|ToString(Rotator) (.Rotation (Math|Transform|BreakTransform Transform)))))

(fn DebugLogScale
  (params (Transform :type Transform))
  (Development|PrintString 0 (Utilities|String|ToString(Vector) (.Scale (Math|Transform|BreakTransform Transform)))))

(fn DebugLogActorInfo
  (params (Actor :type Actor%20Object%20Reference))
  (Development|PrintString 0 (Utilities|String|Append (Utilities|String|Append (Utilities|String|Append (Utilities|GetDisplayName Actor) (Utilities|String|ToString(Integer) (Class|GameplayStatics|GetWorldOriginLocation Actor))) (Utilities|String|ToString(Rotator) (Transformation|GetActorRotation Actor))) (Utilities|String|ToString(Vector) (Transformation|GetActorScale3D Actor)))))

(fn DebugAppendLog
  (params (StrA :type String) (StrB :type String))
  (Development|PrintString 0 (Utilities|String|Append StrA StrB)))

(fn DebugAppendLogBool
  (params (Str :type String) (Bool :type Boolean))
  (Development|PrintString 0 (Utilities|String|Append Str (Utilities|String|ToString(Boolean) Bool))))

(fn DebugAppendLogInt
  (params (Str :type String) (Int :type Integer))
  (Development|PrintString 0 (Utilities|String|Append Str (Utilities|String|ToString(Integer) Int))))

(fn DebugAppendLogFloat
  (params (Str :type String) (Float :type Float%20%28double-precision%29))
  (Development|PrintString 0 (Utilities|String|Append Str (Utilities|String|ToString(Float) Float))))

(fn DebugAppendLogVector
  (params (Str :type String) (Vec :type Vector))
  (Development|PrintString 0 (Utilities|String|Append Str (Utilities|String|ToString(Vector) Vec))))

(fn DebugAppendLogTransform
  (params (Str :type String) (Transform :type Transform))
  (Development|PrintString 0 (Utilities|String|Append Str (Utilities|String|ToString(Transform) Transform))))

(fn DebugAppendLogLocation
  (params (Str :type String) (Transform :type Transform))
  (Development|PrintString 0 (Utilities|String|Append Str (Utilities|String|ToString(Vector) (.Location (Math|Transform|BreakTransform Transform))))))

(fn DebugAppendLogRotation
  (params (Str :type String) (Transform :type Transform))
  (Development|PrintString 0 (Utilities|String|Append Str (Utilities|String|ToString(Rotator) (.Rotation (Math|Transform|BreakTransform Transform))))))

(fn DebugAppendLogScale
  (params (Str :type String) (Transform :type Transform))
  (Development|PrintString 0 (Utilities|String|Append Str (Utilities|String|ToString(Vector) (.Scale (Math|Transform|BreakTransform Transform))))))