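; BP_SphereTank is a player-controllable tank pawn that turns look and move axis inputs into rotation and movement.
; Look axes apply local pitch and yaw rotation directly to the actor rather than to the controller.
; Move axes feed AddMovementInput along the actor's full-rotation forward and right vectors, so movement follows its current pitch as well as heading.
; BeginPlay and the construction script are empty.
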(event Custom|Look%20Up/Down
  (params (Value :type Float%20%28double-precision%29))
  ;[1 1 1] 視点入力：上下
  (Transformation|AddActorLocalRotation (Math|Rotator|MakeRotator 0.0 Value 0.0) false false))

(event Custom|Look%20Right/Left
  (params (Value :type Float%20%28double-precision%29))
  ;[1 1 1] 視点入力：左右
  (Transformation|AddActorLocalRotation (Math|Rotator|MakeRotator 0.0 0.0 Value) false false))

(event Custom|Move%20For/Back%20ward
  (params (Value :type Float%20%28double-precision%29))
  ;[1 1 1] 移動入力：前後
  (Pawn|Input|AddMovementInput (Math|Vector|GetForwardVector (Transformation|GetActorRotation)) Value false))

(event Custom|Move%20Right/Left
  (params (Value :type Float%20%28double-precision%29))
  ;[1 1 1] 移動入力：左右
  (Pawn|Input|AddMovementInput (Math|Vector|GetRightVector (Transformation|GetActorRotation)) Value false))

(event EventBeginPlay)

(fn ConstructionScript)