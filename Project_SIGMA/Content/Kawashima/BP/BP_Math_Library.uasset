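; Blueprint math library providing compound-assignment helpers for integer and float variables.
; Add, subtract, multiply and divide (named Dev) variants each write the result into the by-ref Value and also return it.
; SubAssignInt adds SubValue instead of subtracting it, unlike its float counterpart.
; The divide functions have no explicit zero check.
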(fn AddAssign(Int)
  (params (Value :type Integer%20%28by%20ref%29) (AddValue :type Integer))
  (|SetBy-RefVar Value (+ Value AddValue))
  (return Value))

(fn SubAssign(Int)
  (params (Value :type Integer%20%28by%20ref%29) (SubValue :type Integer))
  (|SetBy-RefVar Value (+ Value SubValue))
  (return Value))

(fn MulAssign(Int)
  (params (Value :type Integer%20%28by%20ref%29) (MulValue :type Integer))
  (|SetBy-RefVar Value (* Value MulValue))
  (return Value))

(fn DevAssign(Int)
  (params (Value :type Integer%20%28by%20ref%29) (DevValue :type Integer))
  (|SetBy-RefVar Value (/ Value DevValue))
  (return Value))

(fn AddAssign(Float)
  (params (Value :type Float%20%28double-precision%29%20%28by%20ref%29) (AddValue :type Float%20%28double-precision%29))
  (|SetBy-RefVar Value (+ Value AddValue))
  (return Value))

(fn SubAssign(Float)
  (params (Value :type Float%20%28double-precision%29%20%28by%20ref%29) (SubValue :type Float%20%28double-precision%29))
  (|SetBy-RefVar Value (- Value SubValue))
  (return Value))

(fn MulAssign(Float)
  (params (Value :type Float%20%28double-precision%29%20%28by%20ref%29) (MulValue :type Float%20%28double-precision%29))
  (|SetBy-RefVar Value (* Value MulValue))
  (return Value))

(fn DevAssign(Float)
  (params (Value :type Float%20%28double-precision%29%20%28by%20ref%29) (DevValue :type Float%20%28double-precision%29))
  (|SetBy-RefVar Value (/ Value DevValue))
  (return Value))