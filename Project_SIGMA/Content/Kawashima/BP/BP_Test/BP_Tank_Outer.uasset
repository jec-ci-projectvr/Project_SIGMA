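; Player-controlled outer body of a rolling sphere tank in an arena shooter, paired with a spawned BP_Tank_Inner cockpit that receives its HP, shield and aim-angle displays.
; Input moves the pawn, spins the sphere mesh, pitches the weapon mount and fires two machineguns along raycast-corrected directions.
; Damage drains shield before HP, with timer-based shield regen that rescales its interval each tick.
; Death notifies the game mode, then restores the player after a delay.
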(event Custom|ReStart
  ;[1 1 1] 死亡後の復活時に呼び出されるイベント
  (Variables|Default|SetCanControl true)
  (Variables|Default|SetIsInvincible false)
  (CallFunction|HealEvent (Math|Float|Truncate (Variables|Default|GetHP_Max)))
  (CallFunction|SetShield (Variables|Default|GetMaxShield))
  (CallFunction|ResetRotate))

(event Custom|EquipWeapons
  (params (RightWeapon :type BP%20Weapon%20Base%20Class%20Reference) (LeftWeapon :type BP%20Weapon%20Base%20Class%20Reference))
  ;[1 1 1] 武器装備をサーバー上で行う
  (CallFunction|EquipLeftWeapon LeftWeapon)
  (CallFunction|EquipRightWeapon RightWeapon))

(event Custom|SetWorldRotation_Multicast)

(event Custom|ResetRotate
  (bind _playerindex (Variables|Default|GetPlayerIndex))
  ;[1 1 1] RPC_回転をリスポーン位置に合わせて初期化する
  (bind _asps_sphere_arena (Utilities|Casting|CastToPS_SphereArena (Game|GetPlayerState _playerindex)))
  (Default|ResetRotate _asps_sphere_arena _playerindex))

(event Custom|SetWeaponAngleonOwningClient
  (params (Val :type Float%20%28double-precision%29))
  (CallFunction|SetWeaponAngle Val))

(event Custom|ReapairShieldEvent_OnServer
  ;[0.1217 0.5041 1] RPCタイマーイベント_シールドの回復
  (CallFunction|RepairShieldEvent))

(event Custom|Player_Dead
  ;[1 0 0] 死亡時イベント
  (CallFunction|DeathEvent)
  (Default|FadeoutMonitor (Variables|Default|GetRef_Inner))
  (Utilities|FlowControl|Delay 5.0)
  (CallFunction|ReStart)
  (Default|FadeinMonitor (Variables|Default|GetRef_Inner)))

(event Custom|Act%20Damage_OnServer
  (params (Damage :type Float%20%28double-precision%29))
  (CallFunction|ActDamage Damage))

(event Custom|ShotEvent
  (params (SpawnPoint :type BPI%20Weapon%20Interface) (shotVelocity :type Vector))
  ;[0.6317 1 0.9501] 射撃イベント
  (Default|Shot SpawnPoint shotVelocity))

(event Custom|SetHPBarOnServer
  ;[1 1 1] HPバーのセット(Multicast)
  (Default|SetHPMaterialMulticast (Variables|Default|GetRef_Inner) (Variables|Default|GetHP_Now) (Variables|Default|GetHP_Max)))

(event Custom|SetShieldBar_OnServer
  ;[1 1 1] シールドバーのセット(Multicast)
  (Default|SetShieldMaterialMulticast (Variables|Default|GetRef_Inner) (Variables|Default|GetCurrentShield) (Variables|Default|GetMaxShield)))

(event Custom|Init_Shield
  ;[0.1248 0.4423 1] シールドの初期化
  (bind _returnvalue (Utilities|Time|SetTimerbyFunctionName 0 "ReapairShieldEvent_OnServer" (Variables|Default|GetShieldInterval) true))
  (Variables|Default|SetShieldTimerHandle _returnvalue))

(event Custom|SetShield
  (params (SetNum :type Float%20%28double-precision%29))
  ;[0.1248 0.4423 1] シールド設定
  (Variables|Default|SetCurrentShield (Math|Float|Min(Float) SetNum (Variables|Default|GetMaxShield)))
  (CallFunction|SetShieldBaronServer)
  (if (<= (Variables|Default|GetCurrentShield) 0.0)
    (CallFunction|ChangeShieldVisibility false)
    (else
      (CallFunction|ChangeShieldVisibility true))))

(event Custom|MoveAudioComponentUpdate
  ;[1 1 1] 移動音の更新
  (Utilities|IfA>B(Float) (Math|Vector|VectorLength (Transformation|GetVelocity)) 0.0
    (:True
      (CallFunction|SetMovingSoundPause false))
    (:False
      (CallFunction|SetMovingSoundPause true))))

(event Custom|StopShotEvent
  (params (Target :type BPI%20Weapon%20Interface))
  (Default|StopShot Target))

(event Custom|ResetAudioListennerPosition
  (Class|PlayerController|SetAudioListenerOverride (Game|GetPlayerController (Variables|Default|GetPlayerIndex)) (Variables|Character|GetMesh) "0, 0, 0" "0, 0, 0"))

(event Custom|ChangeShieldVisibility
  (params (Visibility :type Boolean))
  ;[0.1248 0.4423 1] シールドの可視化変更
  (Rendering|SetVisibility (Variables|Default|GetShield) Visibility false))

(event Custom|HealEvent
  (params (HealValue :type Integer))
  ;[0.577 1 0.6334] RPC_体力回復イベント
  (Variables|Default|SetHP_Now (Math|Float|Min(Float) (+ HealValue (Variables|Default|GetHP_Now)) (Variables|Default|GetHP_Max)))
  (CallFunction|SetHPBaronServer))

(event Custom|OuterAllInitialize
  (bind _ref_inner (Variables|Default|GetRef_Inner))
  (Development|PrintString "StartInitialize")
  (Class|HeadMountedDisplayFunctionLibrary|ResetOrientationandPosition 0.0 "OrientationAndPosition")
  ;[1 1 1] 変数初期化
  (CallFunction|InitValiables 3e+01 5.0 0.4)
  ;[1 1 1] Inner生成
  (bind _asbp_my_game_state_base (Utilities|Casting|CastToBP_MyGameStateBase (Game|GetGameState))
    (:then
      (bind _spawnposition (Default|GetInnerSpawnPoint _asbp_my_game_state_base))
      (CallFunction|InitTankInner _spawnposition)
      ;[1 1 1] InnerのText3D初期化
      (Default|InitTimeText3D _ref_inner)
      (Default|SetHPMaterial _ref_inner (Variables|Default|GetHP_Now) (Variables|Default|GetHP_Max))
      (Default|SetShieldMaterial _ref_inner (Variables|Default|GetCurrentShield) (Variables|Default|GetMaxShield))
      ;[1 1 1] Capture初期化
      (CallFunction|InitCapture)
      ;[1 1 1] ゲームインスタンスから選択した武器を取得
      (bind _asgame_instance (Utilities|Casting|CastToGameInstance (Game|GetGameInstance)))
      (CallFunction|EquipWeapons "/Game/Iino/BP/Actor/Competition/Weapon/BP_Machinegun.BP_Machinegun_C" "/Game/Iino/BP/Actor/Competition/Weapon/BP_Machinegun.BP_Machinegun_C")
      (Rendering|SetVisibility (Variables|Default|GetInSIdeSphere) false false))
    (:CastFailed
      (Development|PrintString "cast failed"))))

(event Custom|PlaySound_Multicast
  (params (Sound :type Sound%20Base%20Object%20Reference) (Location :type Vector))
  ;[1 1 1] サウンドを鳴らす(サーバー、クライアント間共通 )
  (Audio|PlaySoundatLocation Sound Location "0, 0, 0" 1.0 1.0 0.0 0 0 0 0))

(event EventBeginPlay
  (Class|HeadMountedDisplayFunctionLibrary|SetTrackingOrigin "Eye"))

(event EventTakeHit
  (params (Damage :type Integer) (Attacker :type Actor%20Object%20Reference))
  ;[1 0.3005 0.3005] 当たり判定の確認処理　ダメージイベントの呼び出し
  (CallFunction|ActDamageonServer (Math|Conversions|ToFloat(Integer) Damage)))

(event EventTick
  (params (DeltaSeconds :type Float%20%28single-precision%29))
  (CallFunction|MoveAudioComponentUpdate)
  (Transformation|SetWorldRotation (Variables|Default|GetMesh_Sphere) (Variables|Default|GetSphereRot) false false))

(event Input|ActionEvents|InputActionSkill
  (params (Key :type Key%20Structure :default "None"))
  ;[1 1 0.35] シールド生成
  (:Pressed
    (Default|InitSkill (Variables|Default|GetSkill) self)))

(event Input|ActionEvents|InputActionInteract
  (params (Key :type Key%20Structure :default "None"))
  (bind _ref_inner (Variables|Default|GetRef_Inner))
  (bind _vr_character1 (Variables|/Game/Kawashima/BP/BP_Test/BP_Tank_Inner.BP_Tank_Inner_C|GetVR_Character1 _ref_inner))
  ;[1 0.5 1 0.6] アニメーションのオンオフの確認用アクション　状況に応じて再生を行えるかどうかの確認
  (:Pressed
    (Audio|Components|Audio|Play (Variables|/Game/Kawashima/BP/BP_Test/BP_Tank_Inner.BP_Tank_Inner_C|GetSkeletalMesh _ref_inner) false)
    (Audio|Components|Audio|Play (Variables|/Game/Kawashima/BP/BP_Test/BP_Tank_Inner.BP_Tank_Inner_C|GetSkeletalMesh1 _ref_inner) false)
    (Utilities|FlowControl|Delay 1.5)
    (Rendering|SetVisibility _vr_character1 true false)
    (Components|Animation|PlayAnimation _vr_character1 "/Game/Kawashima/VR_3D_Character_v0/Standing_Greeting.Standing_Greeting" false)))

(event Input|ActionEvents|InputActionResetPosition
  (params (Key :type Key%20Structure :default "None"))
  (:Pressed
    (Class|HeadMountedDisplayFunctionLibrary|ResetOrientationandPosition 0.0 "OrientationAndPosition")))

(event Input|AxisEvents|InputAxisTurnRight/LeftMouse
  (params (AxisValue :type Float%20%28single-precision%29))
  ;[0.402 0.3005 0.5972] 視点入力：左右
  (if (Variables|Default|GetCanControl)
    (Pawn|Input|AddControllerYawInput (* AxisValue (Variables|Default|GetLook_Sens)))))

(event Input|AxisEvents|InputAxisLookUp/DownMouse
  (params (AxisValue :type Float%20%28single-precision%29))
  ;[0.4 0.3 0.6] 視点入力：上下
  (CallFunction|SetWeaponAngleonOwningClient (* AxisValue (Variables|Default|GetLook_Sens))))

(event Input|AxisEvents|InputAxisMoveFor/Backward
  (params (AxisValue :type Float%20%28single-precision%29))
  ;[0.402 0.3005 0.5972] 移動入力：前後
  (if (Variables|Default|GetCanControl)
    (Pawn|Input|AddMovementInput (Math|Vector|GetForwardVector (Pawn|GetControlRotation :!class /Script/Engine.Pawn)) (* AxisValue (Variables|Default|GetMove_Speed)) false)
    (Variables|Default|SetSphereRot (Math|Rotator|CombineRotators (Variables|Default|GetSphereRot) (Math|Vector|RotatorfromAxisandAngle (Transformation|GetActorRightVector) (* AxisValue 1.0))))))

(event Input|AxisEvents|InputAxisHoldingFire/Right
  (params (AxisValue :type Float%20%28single-precision%29))
  (bind _cancontrol (Variables|Default|GetCanControl))
  (bind _rightweapon (Variables|Default|GetRightWeapon))
  ;[0.5972 0.8963 1] 射撃：右
  (if (!= AxisValue 0.0)
    (if _cancontrol
      (bind _shotvelocity (CallFunction|Raycast (Variables|Default|GetShootRight)))
      (CallFunction|ShotEvent _rightweapon _shotvelocity))
    (elif _cancontrol
      (CallFunction|StopShotEvent _rightweapon))))

(event Input|AxisEvents|InputAxisMoveRight/Left
  (params (AxisValue :type Float%20%28single-precision%29))
  ;[0.402 0.3005 0.5972] 移動入力：左右
  (if (Variables|Default|GetCanControl)
    (Pawn|Input|AddMovementInput (Math|Vector|GetRightVector (Pawn|GetControlRotation :!class /Script/Engine.Pawn)) (* AxisValue (Variables|Default|GetMove_Speed)) false)
    (Variables|Default|SetSphereRot (Math|Rotator|CombineRotators (Variables|Default|GetSphereRot) (Math|Vector|RotatorfromAxisandAngle (Transformation|GetActorForwardVector) (* AxisValue -1.0))))))

(event Input|AxisEvents|InputAxisHoldingFire/Left
  (params (AxisValue :type Float%20%28single-precision%29))
  (bind _cancontrol (Variables|Default|GetCanControl))
  (bind _leftweapon (Variables|Default|GetLeftWeapon))
  ;[0.5972 0.8963 1] 射撃：左
  (if (!= AxisValue 0.0)
    (if _cancontrol
      (bind _shotvelocity (CallFunction|Raycast (Variables|Default|GetShootLeft)))
      (CallFunction|ShotEvent _leftweapon _shotvelocity))
    (elif _cancontrol
      (CallFunction|StopShotEvent _leftweapon))))

(event Input|KeyboardEvents|Escape
  (params (Key :type Key%20Structure :default "None"))
  ;[1 1 1] ESCキーでタイトルに戻る
  (:Pressed
    (Game|OpenLevel(byObjectReference) "/Game/Kawashima/Title/TitleScreenTestLevel.TitleScreenTestLevel")))

(fn ConstructionScript)

(fn SetWeaponAngle
  (params (Val :type Float%20%28double-precision%29))
  (bind _mesh_weapon (Variables|Default|GetMesh_Weapon))
  (bind _rotmin (LocalVariables|GetRotMin))
  (bind _rotmax (LocalVariables|GetRotMax))
  (bind _matrotmin (LocalVariables|GetMatRotMin))
  (bind _relativerotation (Variables|/Script/Engine.SceneComponent|GetRelativeRotation _mesh_weapon))
  (Transformation|AddLocalRotation _mesh_weapon (Math|Rotator|MakeRotator 0.0 (* Val -1.0) 0.0) false false)
  (Transformation|SetRelativeRotation (Variables|Default|GetMesh_Weapon) (Math|Rotator|MakeRotator 0.0 (Math|Float|Clamp(Float) (.pitch _relativerotation) _rotmin _rotmax) 0.0) false false)
  (Variables|Default|SetParameter%20Value (+ (* (/ (- (.pitch _relativerotation) _rotmin) (- _rotmax _rotmin)) (- (LocalVariables|GetMatRotMax) _matrotmin)) _matrotmin))
  (Rendering|Material|SetScalarParameterValueonMaterials (Variables|/Game/Kawashima/BP/BP_Test/BP_Tank_Inner.BP_Tank_Inner_C|GetMesh_Inside_Forward (Variables|Default|GetRef_Inner)) "TargetAngle" (Variables|Default|GetParameter%20Value)))

(fn InitValiables
  (params (HP :type Float%20%28double-precision%29) (Speed :type Float%20%28double-precision%29) (Sens :type Float%20%28double-precision%29))
  (bind _output_get (Variables|Default|SetHP_Max HP))
  (Variables|Default|SetHP_Now _output_get)
  (Variables|Default|SetMove_Speed Speed)
  (Variables|Default|SetLook_Sens Sens)
  (Variables|Default|SetCurrentShield (Variables|Default|GetMaxShield))
  (Variables|Default|SetShot_Pow 3e+03))

(fn InitTankInner
  (params (SpawnPoint :type Transform))
  (bind _returnvalue (Game|SpawnActorfromClass "/Game/Kawashima/BP/BP_Test/BP_Tank_Inner.BP_Tank_Inner_C" SpawnPoint "Undefined" "MultiplyWithRoot" 0 0))
  (bind _output_get (Variables|Default|SetRef_Inner _returnvalue))
  (Variables|/Game/Kawashima/BP/BP_Test/BP_Tank_Inner.BP_Tank_Inner_C|SetRef_Tank_Outer _output_get self))

(fn InitCapture
  (if (Pawn|IsLocallyControlled)
    (Variables|/Script/Engine.SceneCaptureComponent2D|SetTextureTarget (Variables|Default|GetMain) "/Game/Kawashima/Render_Main.Render_Main") ; メッシュのデフォルト値は空にしておくこと
  ))

(fn SetCamera
  (params (Ref_Inner :type BP%20Tank%20Inner%20Object%20Reference))
  (Game|Player|SetViewTargetwithBlend (Game|GetPlayerController (Variables|Default|GetPlayerIndex)) Ref_Inner 0.0 "VTBlend_Linear" 0.0 false))

(fn ActShot
  (params (SpawnPoint :type Transform))
  (bind _returnvalue (Game|SpawnActorfromClass "/Game/Iino/BP/Actor/Competition/Weapon/Bullet/BP_BulletBase.BP_BulletBase_C" SpawnPoint "Undefined" "MultiplyWithRoot" 0 0))
  (Actor|SetLifeSpan _returnvalue 3.0)
  (Game|Components|ProjectileMovement|SetVelocityinLocalSpace (Variables|/Game/Iino/BP/Actor/Competition/Weapon/Bullet/BP_BulletBase.BP_BulletBase_C|GetProjectileMovement _returnvalue) (* (Math|Vector|MakeVector 1.0 0.0 0.0) (Variables|Default|GetShot_Pow))))

(fn ActDamage
  (params (Damage :type Float%20%28double-precision%29))
  (bind _returnvalue (Transformation|GetActorLocation))
  (if (not (Variables|Default|GetIsInvincible))
    (CallFunction|RestartShieldRepair)
    (Utilities|IfA>B(Float) (Variables|Default|GetCurrentShield) 0.0
      (:True
        (CallFunction|TakeShieldDamage Damage)
        (CallFunction|PlaySoundMulticast "/Game/Iino/Sound/SoundCue/SECue/Shield_TakeHit.Shield_TakeHit" _returnvalue))
      (:False
        (CallFunction|TakeHPDamage Damage)
        (CallFunction|PlaySoundMulticast "/Game/Iino/Sound/SoundCue/SECue/Player_TakeDamage.Player_TakeDamage" _returnvalue)))))

(fn EquipLeftWeapon
  (params (NewWeaponClass :type Actor%20Class%20Reference))
  (bind _returnvalue (Game|SpawnActorfromClass NewWeaponClass (Transformation|GetWorldTransform (Variables|Default|GetShootLeft)) "Undefined" "MultiplyWithRoot" 0 0))
  (bind _asbp_weapon_base (Utilities|Casting|CastToBP_WeaponBase _returnvalue))
  (bind _output_get (Variables|Default|SetLeftWeapon _asbp_weapon_base))
  (Transformation|AttachComponentToComponent (Variables|/Script/Engine.Actor|GetRootComponent _output_get) (Variables|Default|GetshootLeft) "None" "SnapToTarget" "SnapToTarget" "SnapToTarget" true))

(fn EquipRightWeapon
  (params (NewWeaponClass :type Actor%20Class%20Reference))
  (bind _returnvalue (Game|SpawnActorfromClass NewWeaponClass (Transformation|GetWorldTransform (Variables|Default|GetShootRight)) "Undefined" "MultiplyWithRoot" 0 0))
  (bind _asbp_weapon_base (Utilities|Casting|CastToBP_WeaponBase _returnvalue))
  (bind _output_get (Variables|Default|SetRightWeapon _asbp_weapon_base))
  (Transformation|AttachComponentToComponent (Variables|/Script/Engine.Actor|GetRootComponent _output_get) (Variables|Default|GetshootRight) "None" "SnapToTarget" "SnapToTarget" "SnapToTarget" true))

(fn GetNextShieldRecoveryTime
  (params (CurrentInterval :type Float%20%28double-precision%29))
  (return (Math|Float|Max(Float) (* CurrentInterval (LocalVariables|Getfactor)) (LocalVariables|GetminimumInterval))))

(fn RepairShieldEvent
  (Utilities|IfA<B(Float) (Variables|Default|GetCurrentShield) (Variables|Default|GetMaxShield)
    (:True
      (bind _result (Math|Float|IncrementFloat (Variables|Default|GetCurrentShield))
        (:%20%20
          (Utilities|IfA==B(Float) _result 1.0 ; シールドが1に回復した時、シールドを可視化
            (:True
              (CallFunction|ChangeShieldVisibility true))
            (:False
              _))
          (Variables|Default|SetCurrentShield _result)
          (CallFunction|SetShieldBaronServer)
          (bind _newinterval (CallFunction|GetNextShieldRecoveryTime (Variables|Default|GetShieldInterval)))
          (bind _output_get (Variables|Default|SetShieldInterval _newinterval))
          (Utilities|Time|ClearandInvalidateTimerbyHandle (Variables|Default|GetShieldTimerHandle))
          (bind _returnvalue (Utilities|Time|SetTimerbyFunctionName 0 "RepairShieldEvent" _output_get true))
          (Variables|Default|SetShieldTimerHandle _returnvalue))))
    (:False
      (Utilities|Time|ClearandInvalidateTimerbyHandle (Variables|Default|GetShieldTimerHandle)))))

(fn DeathEvent
  (bind _returnvalue (Transformation|GetActorTransform))
  (bind _returnvalue_2 (Game|GetGameMode))
  (bind _self self)
  (Variables|Default|SetIsInvincible true)
  (Variables|Default|SetCanControl false)
  (bind _asbp_domination (Utilities|Casting|CastToBP_Domination _returnvalue_2)
    (:then
      (Audio|PlaySoundatLocation "/Game/Iino/Sound/SoundCue/SECue/PlayerDeath.PlayerDeath" (.location _returnvalue) "0, 0, 0" 1.0 1.0 0.0 0 0 0 0)
      (Default|PlayerDeath _asbp_domination _self))
    (:CastFailed
      (bind _asgm_shootout (Utilities|Casting|CastToGM_Shootout _returnvalue_2))
      (Audio|PlaySoundatLocation "/Game/Iino/Sound/SoundCue/SECue/PlayerDeath.PlayerDeath" (.location _returnvalue) "0, 0, 0" 1.0 1.0 0.0 0 0 0 0)
      (Default|PlayerDeath _asgm_shootout _self))))

(fn RestartShieldRepair
  (bind _initialshieldrepairtime (Variables|Default|GetInitialShieldRepairTime))
  (Utilities|IfA<B(Float) (Variables|Default|GetCurrentShield) (Variables|Default|GetMaxShield)
    (:True
      (Utilities|Time|ClearandInvalidateTimerbyHandle (Variables|Default|GetShieldTimerHandle))
      (bind _returnvalue (Utilities|Time|SetTimerbyFunctionName 0 "RepairShieldEvent" _initialshieldrepairtime true))
      (Variables|Default|SetShieldInterval _initialshieldrepairtime)
      (Variables|Default|SetShieldTimerHandle _returnvalue))))

(fn TakeShieldDamage
  (params (Damage :type Float%20%28double-precision%29))
  (bind _output_get (Variables|Default|SetCurrentShield (Math|Float|Max(Float) (- (Variables|Default|GetCurrentShield) Damage) 0.0)))
  (Utilities|IfA<=B(Float) _output_get 0.0
    (:True
      (CallFunction|ChangeShieldVisibility false))
    (:False
      _))
  (CallFunction|SetShieldBaronServer)
  (Development|PrintString (Utilities|String|Append "シールド残量：" (Utilities|String|ToString(Float) _output_get))))

(fn TakeHPDamage
  (params (Damage :type Float%20%28double-precision%29))
  (bind _output_get (Variables|Default|SetHP_Now (Math|Float|Max(Float) (- (Variables|Default|GetHP_Now) Damage) 0.0)))
  (Utilities|IfA<=B(Float) _output_get 0.0
    (:True
      (CallFunction|PlayerDead))
    (:False
      _))
  (CallFunction|SetHPBaronServer))

(fn SetShieldBar)

(fn TakeHPHeal
  (params (HealValue :type Float%20%28double-precision%29))
  (Variables|Default|SetHP_Now (Math|Float|Min(Float) (+ HealValue (Variables|Default|GetHP_Now)) (Variables|Default|GetHP_Max)))
  (CallFunction|SetHPBaronServer))

(fn IsHPMax
  (return (>= (Variables|Default|GetHP_Now) (Variables|Default|GetHP_Max))))

(fn SetMovingSoundPause
  (params (Condition :type Boolean))
  (Class|AudioComponent|SetPaused (Variables|Default|GetMovingSound) Condition))

(fn SetWeaponAngle0
  (params (Val :type Float%20%28double-precision%29))
  (bind _mesh_weapon (Variables|Default|GetMesh_Weapon))
  (bind _rotmin (LocalVariables|GetRotMin))
  (bind _rotmax (LocalVariables|GetRotMax))
  (bind _matrotmin (LocalVariables|GetMatRotMin))
  (bind _relativerotation (Variables|/Script/Engine.SceneComponent|GetRelativeRotation _mesh_weapon))
  (Transformation|AddLocalRotation _mesh_weapon (Math|Rotator|MakeRotator 0.0 (* Val -1.0) 0.0) false false)
  (Transformation|SetRelativeRotation (Variables|Default|GetMesh_Weapon) (Math|Rotator|MakeRotator 0.0 (Math|Float|Clamp(Float) (.pitch _relativerotation) _rotmin _rotmax) 0.0) false false)
  (Rendering|Material|SetScalarParameterValueonMaterials (Variables|/Game/Kawashima/BP/BP_Test/BP_Tank_Inner.BP_Tank_Inner_C|GetMesh_Inside_Forward (Variables|Default|GetRef_Inner)) "TargetAngle" (+ (* (/ (- (.pitch _relativerotation) _rotmin) (- _rotmax _rotmin)) (- (LocalVariables|GetMatRotMax) _matrotmin)) _matrotmin)))

(fn Raycast
  (params (StartArrow :type Arrow%20Component%20Object%20Reference))
  (bind _returnvalue (Math|Vector|GetForwardVector StartArrow))
  (bind _rayarrow (Variables|Default|GetRayArrow))
  (bind _returnvalue_2 (Transformation|GetWorldLocation _rayarrow))
  (bind _outhit (Collision|LineTraceByChannel _returnvalue_2 (+ _returnvalue_2 (* (Math|Vector|GetForwardVector _rayarrow) 6e+03)) "TraceTypeQuery1" false 0 "ForOneFrame"))
  (bind _output_get (Variables|Default|SetOut%20Hit%20Location (.location _outhit)))
  (return (Math|Vector|MakeVector (.x (Math|Vector|RotateVector (Math|Vector|MakeVector 1.0 0.0 0.0) (Math|Vector|RotatorfromAxisandAngle (Math|Vector|VectorUp) (Class|KismetMathLibrary|DegAcos (Math|Vector|DotProduct (Math|Vector|Normalize (- _output_get (Transformation|GetWorldLocation StartArrow))) _returnvalue))))) (* (.y (Math|Vector|RotateVector (Math|Vector|MakeVector 1.0 0.0 0.0) (Math|Vector|RotatorfromAxisandAngle (Math|Vector|VectorUp) (Class|KismetMathLibrary|DegAcos (Math|Vector|DotProduct (Math|Vector|Normalize (- _output_get (Transformation|GetWorldLocation StartArrow))) _returnvalue))))) -1.0 (/ (.z (Math|Vector|CrossProduct (Math|Vector|Normalize (- _output_get (Transformation|GetWorldLocation StartArrow))) _returnvalue)) (Math|Float|Absolute(Float) (.z (Math|Vector|CrossProduct (Math|Vector|Normalize (- _output_get (Transformation|GetWorldLocation StartArrow))) _returnvalue))))) (.z (Math|Vector|RotateVector (Math|Vector|MakeVector 1.0 0.0 0.0) (Math|Vector|RotatorfromAxisandAngle (Math|Vector|VectorUp) (Class|KismetMathLibrary|DegAcos (Math|Vector|DotProduct (Math|Vector|Normalize (- _output_get (Transformation|GetWorldLocation StartArrow))) _returnvalue))))))))