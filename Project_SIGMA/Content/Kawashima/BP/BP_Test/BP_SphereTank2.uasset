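; Player pawn for a networked VR arena shooter: a rolling sphere tank with in-cockpit HP, score, timer and radar displays.
; Input moves and spins the sphere and fires two attached weapons (hard-coded Bazooka and Shotgun), corrected toward a center-ray trace.
; Damage restarts the looping auto-heal timer; death notifies GM_Shootout, fades, then respawns with a timed invincibility shield.
; Server/Multicast events replicate effects and display updates.
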(event Custom|SpawnDisolveEffect_Multicast
  (bind _returnvalue (Transformation|GetActorLocation))
  (bind (_x _y _z) (Class|KismetMathLibrary|BreakVector3f _returnvalue))
  ;[1 1 1] 死亡時のエフェクト
  (Niagara|SpawnSystematLocation "/TeleportVFX/Teleportation_VFX/Particles/P_TeleportDissolve_01.P_TeleportDissolve_01" (Math|Vector|MakeVector _x _y (- _z 1e+02)) "0, 0, 0" "1.500000,1.500000,1.500000"))

(event Custom|SpawnDisolveEffect_OnServer
  ;[1 1 1] 死亡時のエフェクト
  (CallFunction|SpawnDisolveEffectMulticast))

(event Custom|AutoHealEvent
  (Development|PrintString "自動回復")
  (CallFunction|TakeHPHeal (Variables|Default|GetAutoHealValue)))

(event Custom|InvincibleShieldEnable
  (CallFunction|SetShieldVisible true)
  (Variables|Default|SetIsInvincible true)
  (bind _returnvalue (Utilities|Time|SetTimerbyFunctionName 0 "InvincibleShieldDisable" (Variables|Default|GetInvinsibleShieldTime)))
  (Variables|Default|SetTimer _returnvalue))

(event Custom|SetWeaponAngleonOwningClient
  (params (Val :type Float%20%28double-precision%29))
  (CallFunction|SetWeaponAngle Val))

(event Custom|InvincibleShieldDisable
  (CallFunction|SetShieldVisible false)
  (Variables|Default|SetIsInvincible false))

(event Custom|SetShieldVisible
  (params (bNewVisibility :type Boolean))
  (Rendering|SetVisibility (Variables|Default|GetInvincibleShield) bNewVisibility false))

(event Custom|Player_Dead
  ;[1 0 0] 死亡時イベント
  (CallFunction|DeathEvent)
  (CallFunction|FadeOut)
  (Utilities|FlowControl|Delay 3.0)
  (CallFunction|ReStart)
  (CallFunction|Fadein))

(event Custom|Act%20Damage_OnServer
  (params (Damage :type Float%20%28double-precision%29))
  (CallFunction|ActDamage Damage))

(event Custom|UpdateScoraGauge_Multicast
  ;[1 0.4605 0.5505] Inner移植
  ;;[1 1 1] ゲージ操作のための関数
  (CallFunction|UpdateScoreGauge))

(event Custom|SetHPBarOnServer
  ;[1 1 1] HPバーのセット(Multicast)
  (Rendering|Material|SetScalarParameterValueonMaterials (Variables|Default|GetMesh_HP) "Value" (/ (Variables|Default|GetHP%20Now) (Variables|Default|GetHP_Max))))

(event Custom|UpdateScoreGauge_OnServer
  ;[1 0.4605 0.5505] Inner移植
  ;;[1 1 1] ゲージ操作のための関数
  (CallFunction|UpdateScoraGaugeMulticast))

(event Custom|ReStart
  ;[1 1 1] 死亡後の復活時に呼び出されるイベント
  (Variables|Default|SetCanControl true)
  (Variables|Default|SetIsInvincible false)
  (CallFunction|Fadein)
  (CallFunction|RespawnEffectonServer)
  (CallFunction|HealEvent (Math|Float|Truncate (Variables|Default|GetHP_Max)))
  (CallFunction|ResetRotate)
  (CallFunction|InvincibleShieldEnable))

(event Custom|ShotEvent
  (params (SpawnPoint :type BPI%20Weapon%20Interface) (shotVelocity :type Vector))
  ;[0.6317 1 0.9501] 射撃イベント
  (Default|Shot SpawnPoint shotVelocity))

(event Custom|MoveAudioComponentUpdate
  ;[1 1 1] 移動音の更新
  (Utilities|IfA>B(Float) (Math|Vector|VectorLength (Transformation|GetVelocity)) 0.0
    (:True
      (CallFunction|SetMovingSoundPause false))
    (:False
      (CallFunction|SetMovingSoundPause true))))

(event Custom|HealEvent
  (params (HealValue :type Integer))
  ;[0.577 1 0.6334] RPC_体力回復イベント
  (Variables|Default|SetHP%20Now (Math|Float|Min(Float) (+ HealValue (Variables|Default|GetHP%20Now)) (Variables|Default|GetHP_Max)))
  (CallFunction|SetHPBaronServer))

(event Custom|Initialize
  (Development|PrintString "StartInitialize")
  (Class|HeadMountedDisplayFunctionLibrary|ResetOrientationandPosition 0.0 "OrientationAndPosition")
  ;[1 1 1] 変数初期化
  (CallFunction|InitValiables 5e+01 5.0 0.4)
  ;[1 1 1] InnerのText3D初期化
  (CallFunction|InittimeText3D)
  (CallFunction|SetHPMaterial (Variables|Default|GetHP%20Now) (Variables|Default|GetHP_Max))
  ;[1 1 1] Capture初期化
  (CallFunction|InitCapture)
  ;[1 1 1] ゲームインスタンスから選択した武器を取得
  (bind _asgame_instance (Utilities|Casting|CastToGameInstance (Game|GetGameInstance)))
  (CallFunction|EquipWeapons "/Game/Iino/BP/Actor/Competition/Weapon/BP_Bazooka.BP_Bazooka_C" "/Game/Iino/BP/Actor/Competition/Weapon/BP_Shotgun.BP_Shotgun_C")
  (CallFunction|Fadein)
  (bind _returnvalue (Utilities|Time|SetTimerbyFunctionName 0 "AutoHealEvent" (Variables|Default|GetAutoHealInterval) true))
  (Variables|Default|SetAutoHealTimer _returnvalue))

(event Custom|EquipWeapons
  (params (RightWeapon :type BP%20Weapon%20Base%20Class%20Reference) (LeftWeapon :type BP%20Weapon%20Base%20Class%20Reference))
  ;[1 1 1] 武器装備をサーバー上で行う
  (CallFunction|EquipLeftWeapon LeftWeapon)
  (CallFunction|EquipRightWeapon RightWeapon))

(event Custom|RespawnEffect_OnServer
  ;[1 1 1] リスポーン時のエフェクト
  (CallFunction|RespawnEffectMulticast))

(event Custom|StopShotEvent
  (params (Target :type BPI%20Weapon%20Interface))
  (Default|StopShot Target))

(event Custom|PlaySound_Multicast
  (params (Sound :type Sound%20Base%20Object%20Reference) (Location :type Vector))
  ;[1 1 1] サウンドを鳴らす(サーバー、クライアント間共通 )
  (Audio|PlaySoundatLocation Sound Location "0, 0, 0" 1.0 1.0 0.0 0 0 0 0))

(event Custom|ResetRotate
  (bind _player_index (Variables|Default|GetPlayer%20Index))
  ;[1 1 1] RPC_回転をリスポーン位置に合わせて初期化する
  (bind _asps_sphere_arena (Utilities|Casting|CastToPS_SphereArena (Game|GetPlayerState _player_index)))
  (Default|ResetRotate _asps_sphere_arena _player_index))

(event Custom|FadeIn
  ;[1 1 1] 乗り物のフェード
  (bind _fade (Timeline|タイムライン_2 PlayFromStart)
    (:Update
      (Rendering|Material|SetScalarParameterValueonMaterials (Variables|Default|GetMesh_Inside_Forward) "Alpha" (Math|Float|Lerp 1.0 0.0 _fade)))))

(event Custom|FadeOut
  ;[1 1 1] 乗り物のフェード
  (bind _fade (Timeline|タイムライン_1 PlayFromStart)
    (:Update
      (Rendering|Material|SetScalarParameterValueonMaterials (Variables|Default|GetMesh_Inside_Forward) "Alpha" _fade))))

(event Custom|SetHPMaterial_Multicast
  (params (HP_Now :type Float%20%28double-precision%29) (HP_Max :type Float%20%28double-precision%29))
  ;[1 0.4605 0.5505] Inner移植
  ;;[1 1 1] HPゲージの更新(Multicast)
  (CallFunction|SetHPMaterial HP_Now HP_Max))

(event Custom|RespawnEffect_Multicast
  (bind _returnvalue (Transformation|GetActorLocation))
  (bind (_x _y _z) (Class|KismetMathLibrary|BreakVector3f _returnvalue))
  ;[1 1 1] リスポーン時のエフェクト
  (Niagara|SpawnSystematLocation "/TeleportVFX/Teleportation_VFX/Particles/P_TeleportSpawn_01.P_TeleportSpawn_01" (Math|Vector|MakeVector _x _y (- _z 1e+02)) "0, 0, 0" "1.500000,1.500000,1.500000"))

(event Custom|UpdateRader_Multicast
  (bind _self self)
  ;[1 0.4605 0.5505] Inner移植
  (Utilities|IsValid _self
    (:Is%20Valid
      (Default|UpdateRader (Variables|Default|GetRader) _self))))

(event Custom|UpdateRader_OnServer
  ;[1 0.4605 0.5505] Inner移植
  (CallFunction|UpdateRaderMulticast))

(event Custom|HealEvent_OnServer
  (params (HealValue :type Float%20%28double-precision%29))
  (CallFunction|TakeHPHeal HealValue))

(event EventTick
  (params (DeltaSeconds :type Float%20%28single-precision%29))
  (CallFunction|MoveAudioComponentUpdate)
  (Transformation|SetWorldRotation (Variables|Default|GetMesh_Sphere) (Variables|Default|GetSphereRot) false false)
  ;[0 0 1] タイマー処理
  (CallFunction|UpdateTimer)
  ;[0 1 1] 戦況ゲージ更新処理(サーバーからRPC)
  (CallFunction|UpdateScoreGaugeonServer))

(event EventTakeHit
  (params (Damage :type Integer) (Attacker :type Actor%20Object%20Reference))
  ;[1 0.3005 0.3005] 当たり判定の確認処理　ダメージイベントの呼び出し
  (CallFunction|ActDamageonServer (Math|Conversions|ToFloat(Integer) Damage)))

(event EventBeginPlay
  (Class|HeadMountedDisplayFunctionLibrary|SetTrackingOrigin "Eye"))

(event Input|ActionEvents|InputActionInteract
  (params (Key :type Key%20Structure :default "None"))
  (bind _vr_character1 (Variables|Default|GetVR_Character1))
  ;[1 0.5 1 0.6] アニメーションのオンオフの確認用アクション　状況に応じて再生を行えるかどうかの確認
  (:Pressed
    (Audio|Components|Audio|Play (Variables|Default|GetSkeletalMesh) false)
    (Audio|Components|Audio|Play (Variables|Default|GetSkeletalMesh1) false)
    (Utilities|FlowControl|Delay 5.0)
    (Rendering|SetVisibility _vr_character1 true false)
    (Components|Animation|PlayAnimation _vr_character1 "/Game/Kawashima/VR_3D_Character_v0/Standing_Greeting.Standing_Greeting" false)))

(event Input|ActionEvents|InputActionResetPosition
  (params (Key :type Key%20Structure :default "None"))
  (:Pressed
    (Class|HeadMountedDisplayFunctionLibrary|ResetOrientationandPosition 0.0 "OrientationAndPosition")))

(event Input|AxisEvents|InputAxisTurnRight/LeftMouse
  (params (AxisValue :type Float%20%28single-precision%29))
  ;[0.402 0.3005 0.5972] 視点入力：左右
  (if (Variables|Default|GetCanControl)
    (Pawn|Input|AddControllerYawInput (* AxisValue (Variables|Default|GetLook_Sens)))))

(event Input|AxisEvents|InputAxisLookUp/DownMouse
  (params (AxisValue :type Float%20%28single-precision%29))
  ;[0.4 0.3 0.6] 視点入力：上下
  (CallFunction|SetWeaponAngleonOwningClient (* AxisValue (Variables|Default|GetLook_Sens))))

(event Input|AxisEvents|InputAxisMoveFor/Backward
  (params (AxisValue :type Float%20%28single-precision%29))
  ;[0.402 0.3005 0.5972] 移動入力：前後
  (if (Variables|Default|GetCanControl)
    (Pawn|Input|AddMovementInput (Math|Vector|GetForwardVector (Pawn|GetControlRotation :!class /Script/Engine.Pawn)) (* AxisValue (Variables|Default|GetMove_Speed)) false)
    (Variables|Default|SetSphereRot (Math|Rotator|CombineRotators (Variables|Default|GetSphereRot) (Math|Vector|RotatorfromAxisandAngle (Transformation|GetActorRightVector) (* AxisValue 1.0))))))

(event Input|AxisEvents|InputAxisHoldingFire/Right
  (params (AxisValue :type Float%20%28single-precision%29))
  (bind _cancontrol (Variables|Default|GetCanControl))
  (bind _rightweapon (Variables|Default|GetRightWeapon))
  ;[0.5972 0.8963 1] 射撃：右
  (if (!= AxisValue 0.0)
    (if _cancontrol
      (bind _shotvelocity (CallFunction|Raycast (Variables|Default|GetShootRight)))
      (CallFunction|ShotEvent _rightweapon _shotvelocity))
    (elif _cancontrol
      (CallFunction|StopShotEvent _rightweapon))))

(event Input|AxisEvents|InputAxisMoveRight/Left
  (params (AxisValue :type Float%20%28single-precision%29))
  ;[0.402 0.3005 0.5972] 移動入力：左右
  (if (Variables|Default|GetCanControl)
    (Pawn|Input|AddMovementInput (Math|Vector|GetRightVector (Pawn|GetControlRotation :!class /Script/Engine.Pawn)) (* AxisValue (Variables|Default|GetMove_Speed)) false)
    (Variables|Default|SetSphereRot (Math|Rotator|CombineRotators (Variables|Default|GetSphereRot) (Math|Vector|RotatorfromAxisandAngle (Transformation|GetActorForwardVector) (* AxisValue -1.0))))))

(event Input|AxisEvents|InputAxisHoldingFire/Left
  (params (AxisValue :type Float%20%28single-precision%29))
  (bind _cancontrol (Variables|Default|GetCanControl))
  (bind _leftweapon (Variables|Default|GetLeftWeapon))
  ;[0.5972 0.8963 1] 射撃：左
  (if (!= AxisValue 0.0)
    (if _cancontrol
      (bind _shotvelocity (CallFunction|Raycast (Variables|Default|GetShootLeft)))
      (CallFunction|ShotEvent _leftweapon _shotvelocity))
    (elif _cancontrol
      (CallFunction|StopShotEvent _leftweapon))))

(event Input|KeyboardEvents|Escape
  (params (Key :type Key%20Structure :default "None"))
  ;[1 1 1] ESCキーでタイトルに戻る
  (:Pressed
    (Game|OpenLevel(byObjectReference) "/Game/Kawashima/Title/TitleScreenTestLevel.TitleScreenTestLevel")))

(fn ConstructionScript)

(fn InitValiables
  (params (HP :type Float%20%28double-precision%29) (Speed :type Float%20%28double-precision%29) (Sens :type Float%20%28double-precision%29))
  (bind _output_get (Variables|Default|SetHP_Max HP))
  (Variables|Default|SetHP%20Now _output_get)
  (Variables|Default|SetMove_Speed Speed)
  (Variables|Default|SetLook_Sens Sens))

(fn InitTankInner
  (params (SpawnPoint :type Transform)))

(fn InitCapture)

(fn EquipLeftWeapon
  (params (NewWeaponClass :type Actor%20Class%20Reference))
  (bind _returnvalue (Game|SpawnActorfromClass NewWeaponClass (Transformation|GetWorldTransform (Variables|Default|GetShootLeft)) "Undefined" "MultiplyWithRoot" self 0))
  (bind _asbp_weapon_base (Utilities|Casting|CastToBP_WeaponBase _returnvalue))
  (bind _output_get (Variables|Default|SetLeftWeapon _asbp_weapon_base))
  (Transformation|AttachComponentToComponent (Variables|/Script/Engine.Actor|GetRootComponent _output_get) (Variables|Default|GetshootLeft) "None" "SnapToTarget" "SnapToTarget" "SnapToTarget" true))

(fn EquipRightWeapon
  (params (NewWeaponClass :type Actor%20Class%20Reference))
  (bind _returnvalue (Game|SpawnActorfromClass NewWeaponClass (Transformation|GetWorldTransform (Variables|Default|GetShootRight)) "Undefined" "MultiplyWithRoot" self 0))
  (bind _asbp_weapon_base (Utilities|Casting|CastToBP_WeaponBase _returnvalue))
  (bind _output_get (Variables|Default|SetRightWeapon _asbp_weapon_base))
  (Transformation|AttachComponentToComponent (Variables|/Script/Engine.Actor|GetRootComponent _output_get) (Variables|Default|GetshootRight) "None" "SnapToTarget" "SnapToTarget" "SnapToTarget" true))

(fn ActDamage
  (params (Damage :type Float%20%28double-precision%29))
  (if (Variables|Default|GetIsInvincible)
    (CallFunction|PlaySoundMulticast "/Game/Iino/Sound/SoundCue/SECue/Shield_TakeHit.Shield_TakeHit" (Transformation|GetActorLocation))
    (else
      (Utilities|Time|ClearandInvalidateTimerbyHandle (Variables|Default|GetAutoHealTimer))
      (bind _returnvalue (Utilities|Time|SetTimerbyFunctionName 0 "AutoHealEvent" (Variables|Default|GetAutoHealInterval) true))
      (Variables|Default|SetAutoHealTimer _returnvalue)
      (CallFunction|TakeHPDamage Damage)
      (CallFunction|PlaySoundMulticast "/Game/Iino/Sound/SoundCue/SECue/Player_TakeDamage.Player_TakeDamage" (Transformation|GetActorLocation)))))

(fn DeathEvent
  (Variables|Default|SetIsInvincible true)
  (Variables|Default|SetCanControl false)
  (CallFunction|FadeOut)
  (bind _asgm_shootout (Utilities|Casting|CastToGM_Shootout (Game|GetGameMode)))
  (Audio|PlaySoundatLocation "/Game/Iino/Sound/SoundCue/SECue/PlayerDeath.PlayerDeath" (.location (Transformation|GetActorTransform)) "0, 0, 0" 1.0 1.0 0.0 0 0 0 0)
  (CallFunction|SpawnDisolveEffectonServer)
  (Default|PlayerDeath _asgm_shootout self))

(fn SetMovingSoundPause
  (params (Condition :type Boolean))
  (Class|AudioComponent|SetPaused (Variables|Default|GetMovingSound) Condition))

(fn UpdateScoreGauge
  (bind _asps_sphere_arena (Utilities|Casting|CastToPS_SphereArena (Game|GetPlayerState (Variables|Default|GetPlayer%20Index))))
  (bind _score (Default|GetPlayerScore _asps_sphere_arena))
  (Rendering|Material|SetScalarParameterValueonMaterials (Variables|Default|GetMesh_Table) "Value" (- 1e+02 (Math|Conversions|ToFloat(Integer) _score))))

(fn UpdateTimer
  (bind _ref_timetext3d (Variables|Default|GetRef_TimeText3D))
  (bind _asbp_my_game_state_base (Utilities|Casting|CastToBP_MyGameStateBase (Game|GetGameState)))
  (Utilities|IsValid _ref_timetext3d
    (:Is%20Valid
      (Default|SetTime _ref_timetext3d (Math|Float|Truncate (Variables|/Game/Iino/BP/GameState/BP_MyGameStateBase.BP_MyGameStateBase_C|GetTimeLimit _asbp_my_game_state_base))) ; 秒での経過時間ないし残り時間を渡す
    )))

(fn SetHPMaterial
  (params (HP_Now :type Float%20%28double-precision%29) (HP_Max :type Float%20%28double-precision%29))
  (Rendering|Material|SetScalarParameterValueonMaterials (Variables|Default|GetMesh_HP) "Value" (/ HP_Now HP_Max)))

(fn InitCamera)

(fn InittimeText3D
  (bind _asbp_time_text_3d (Utilities|Casting|CastToBP_TimeText3D (Variables|/Script/Engine.ChildActorComponent|GetChildActor (Variables|Default|GetBP_TimeText3D))))
  (Variables|Default|SetRef_TimeText3D _asbp_time_text_3d))

(fn SetHPMaterial
  (params (HPNow :type Float%20%28double-precision%29) (HPMax :type Float%20%28double-precision%29))
  (Rendering|Material|SetScalarParameterValueonMaterials (Variables|Default|GetMesh_HP) "Value" (/ HPNow HPMax)))

(fn Raycast
  (params (StartArrow :type Arrow%20Component%20Object%20Reference))
  (bind _returnvalue (Transformation|GetWorldLocation StartArrow))
  (bind _returnvalue_2 (Math|Vector|GetForwardVector StartArrow))
  (bind _rayarrow (Variables|Default|GetRayArrow))
  (bind _returnvalue_3 (Transformation|GetWorldLocation _rayarrow))
  (bind _outhit (Collision|LineTraceByChannel _returnvalue_3 (+ _returnvalue_3 (* (Math|Vector|GetForwardVector _rayarrow) 6e+03)) "TraceTypeQuery1" false 0 "None"))
  (if (.bblockinghit _outhit)
    ;[1 1 1] レイがオブジェクトに当たった時の処理
    (bind _output_get (Variables|Default|SetOut%20Hit%20Location (.location _outhit)))
    (return (Math|Vector|MakeVector (.x (Math|Vector|RotateVector (Math|Vector|MakeVector 1.0 0.0 0.0) (Math|Vector|RotatorfromAxisandAngle (Math|Vector|VectorUp) (Class|KismetMathLibrary|DegAcos (Math|Vector|DotProduct (Math|Vector|Normalize (- _output_get _returnvalue)) _returnvalue_2))))) (* (.y (Math|Vector|RotateVector (Math|Vector|MakeVector 1.0 0.0 0.0) (Math|Vector|RotatorfromAxisandAngle (Math|Vector|VectorUp) (Class|KismetMathLibrary|DegAcos (Math|Vector|DotProduct (Math|Vector|Normalize (- _output_get _returnvalue)) _returnvalue_2))))) -1.0 (/ (.z (Math|Vector|CrossProduct (Math|Vector|Normalize (- _output_get _returnvalue)) _returnvalue_2)) (Math|Float|Absolute(Float) (.z (Math|Vector|CrossProduct (Math|Vector|Normalize (- _output_get _returnvalue)) _returnvalue_2))))) (.z (Math|Vector|RotateVector (Math|Vector|MakeVector 1.0 0.0 0.0) (Math|Vector|RotatorfromAxisandAngle (Math|Vector|VectorUp) (Class|KismetMathLibrary|DegAcos (Math|Vector|DotProduct (Math|Vector|Normalize (- _output_get _returnvalue)) _returnvalue_2)))))))
    (else
      ;[1 1 1] レイがオブジェクトに当たらなかった時の処理
      (bind _output_get_2 (Variables|Default|SetOut%20Hit%20Location (.traceend _outhit))) ; レイの終わりの座標
      (return (Math|Vector|MakeVector (.x (Math|Vector|RotateVector (Math|Vector|MakeVector 1.0 0.0 0.0) (Math|Vector|RotatorfromAxisandAngle (Math|Vector|VectorUp) (Class|KismetMathLibrary|DegAcos (Math|Vector|DotProduct (Math|Vector|Normalize (- _output_get_2 _returnvalue)) _returnvalue_2))))) (* (.y (Math|Vector|RotateVector (Math|Vector|MakeVector 1.0 0.0 0.0) (Math|Vector|RotatorfromAxisandAngle (Math|Vector|VectorUp) (Class|KismetMathLibrary|DegAcos (Math|Vector|DotProduct (Math|Vector|Normalize (- _output_get_2 _returnvalue)) _returnvalue_2))))) -1.0 (/ (.z (Math|Vector|CrossProduct (Math|Vector|Normalize (- _output_get_2 _returnvalue)) _returnvalue_2)) (Math|Float|Absolute(Float) (.z (Math|Vector|CrossProduct (Math|Vector|Normalize (- _output_get_2 _returnvalue)) _returnvalue_2))))) (.z (Math|Vector|RotateVector (Math|Vector|MakeVector 1.0 0.0 0.0) (Math|Vector|RotatorfromAxisandAngle (Math|Vector|VectorUp) (Class|KismetMathLibrary|DegAcos (Math|Vector|DotProduct (Math|Vector|Normalize (- _output_get_2 _returnvalue)) _returnvalue_2))))))))))

(fn SetWeaponAngle
  (params (Val :type Float%20%28double-precision%29))
  (bind _mesh_weapon (Variables|Default|GetMesh_Weapon))
  (Transformation|AddLocalRotation _mesh_weapon (Math|Rotator|MakeRotator 0.0 (* Val -1.0) 0.0) false false)
  (Transformation|SetRelativeRotation (Variables|Default|GetMesh_Weapon) (Math|Rotator|MakeRotator 0.0 (Math|Float|Clamp(Float) (.pitch (Variables|/Script/Engine.SceneComponent|GetRelativeRotation _mesh_weapon)) (LocalVariables|GetRotMin) (LocalVariables|GetRotMax)) 0.0) false false))

(fn TakeHPDamage
  (params (Damage :type Float%20%28double-precision%29))
  (bind _output_get (Variables|Default|SetHP%20Now (Math|Float|Max(Float) (- (Variables|Default|GetHP%20Now) Damage) 0.0)))
  (Utilities|IfA<=B(Float) _output_get 0.0
    (:True
      (CallFunction|PlayerDead))
    (:False
      _))
  (CallFunction|SetHPBaronServer))

(fn IsHPMax
  (return (>= (Variables|Default|GetHP%20Now) (Variables|Default|GetHP_Max))))

(fn TakeHPHeal
  (params (HealValue :type Float%20%28double-precision%29))
  (Variables|Default|SetHP%20Now (Math|Float|Min(Float) (+ HealValue (Variables|Default|GetHP%20Now)) (Variables|Default|GetHP_Max)))
  (CallFunction|SetHPBaronServer))

(fn GetTeamID
  (return (Variables|Default|GetTeam%20ID)))