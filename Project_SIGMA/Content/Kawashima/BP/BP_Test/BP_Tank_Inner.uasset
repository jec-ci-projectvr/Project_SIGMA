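; BP_Tank_Inner is the VR cockpit interior of a tank, displaying the outer tank's view, radar, timer and gauges.
; A looping timer refreshes the child-actor radar and Tick updates the match timer and score gauge, with radar and score relayed through server-to-multicast events.
; HP, shield, score and front-monitor fades drive mesh material parameters.
; The outer tank's capture render target is assigned only when locally controlled, as a bug workaround.
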(event Custom|UpdateRaderEvent
  ;[0.5896 0.2389 1] レーダーの更新
  (CallFunction|UpdateRaderonServer))

(event Custom|FadeoutMonitor
  ;[1 1 1] 前面モニタのフェードアウト
  (bind _fade (Timeline|Timeline Play)
    (:Update
      (Rendering|Material|SetScalarParameterValueonMaterials (Variables|Default|GetMesh_Inside_Forward) "BlackFilter" _fade))))

(event Custom|ResetRaderAngle_Multicast
  (bind _asbp_rader (Utilities|Casting|CastToBP_Rader (Variables|/Script/Engine.ChildActorComponent|GetChildActor (Variables|Default|GetBP_Rader))))
  (bind _asps_sphere_arena (Utilities|Casting|CastToPS_SphereArena (Game|GetPlayerState (Variables|/Game/Kawashima/BP/BP_Test/BP_Tank_Outer.BP_Tank_Outer_C|GetPlayerIndex (Variables|Default|GetRef_Tank_Outer)))))
  (Variables|/Game/Kawashima/BP/BP_Rader.BP_Rader_C|SetBaseAngle _asbp_rader (+ (.Yaw (Math|Rotator|BreakRotator (.rotation (Variables|/Game/Iino/BP/PlayerState/PS_SphereArena.PS_SphereArena_C|GetRespawnTransform _asps_sphere_arena)))) 1.8e+02)))

(event Custom|UpdateScoraGauge_Multicast
  ;[1 1 1] ゲージ操作のための関数
  (CallFunction|UpdateScoreGauge))

(event Custom|UpdateScoreGauge_OnServer
  ;[1 1 1] ゲージ操作のための関数
  (CallFunction|UpdateScoraGaugeMulticast))

(event Custom|FadeInMonitor
  ;[1 1 1] 前面モニタのフェードイン
  (bind _fade (Timeline|Timeline_0 Play)
    (:Update
      (Rendering|Material|SetScalarParameterValueonMaterials (Variables|Default|GetMesh_Inside_Forward) "BlackFilter" (Math|Float|Lerp 1.0 0.0 _fade)))))

(event Custom|SetHPMaterial_Multicast
  (params (HP_Now :type Float%20%28double-precision%29) (HP_Max :type Float%20%28double-precision%29))
  ;[1 1 1] HP,シールドゲージの更新(Multicast)
  (CallFunction|SetHPMaterial HP_Now HP_Max))

(event Custom|SetShieldMaterial_Multicast
  (params (CurrentShield :type Float%20%28double-precision%29) (MaxShield :type Float%20%28double-precision%29))
  ;[1 1 1] HP,シールドゲージの更新(Multicast)
  (CallFunction|SetShieldMaterial CurrentShield MaxShield))

(event Custom|UpdateRader_Multicast
  (bind _ref_tank_outer (Variables|Default|GetRef_Tank_Outer))
  (Utilities|IsValid _ref_tank_outer
    (:Is%20Valid
      (Default|UpdateRader (Variables|Default|GetRader) _ref_tank_outer (Variables|Default|GetRaderTarget)))))

(event Custom|UpdateRader_OnServer
  (CallFunction|UpdateRaderMulticast))

(event Custom|ResetRaderAngle
  (CallFunction|ResetRaderAngleMulticast))

(event EventBeginPlay
  (bind _asbp_rader (Utilities|Casting|CastToBP_Rader (Variables|/Script/Engine.ChildActorComponent|GetChildActor (Variables|Default|GetBP_Rader))))
  (Variables|Default|SetRader _asbp_rader)
  (Utilities|Time|SetTimerbyFunctionName 0 "UpdateRaderEvent" 0.1 true)
  (Utilities|FlowControl|Delay 1.0)
  (bind _asps_sphere_arena (Utilities|Casting|CastToPS_SphereArena (Game|GetPlayerState (Variables|/Game/Kawashima/BP/BP_Test/BP_Tank_Outer.BP_Tank_Outer_C|GetPlayerIndex (Variables|Default|GetRef_Tank_Outer)))))
  (Variables|Default|SetRef_PlayerState _asps_sphere_arena)
  (Utilities|FlowControl|Delay 2.0)
  (CallFunction|FadeinMonitor))

(event EventTick
  (params (DeltaSeconds :type Float%20%28single-precision%29))
  ;[0 0 1] テスト用タイマー処理
  (CallFunction|UpdateTimer)
  ;[0 1 1] 戦況ゲージ更新処理(サーバーからRPC)
  (CallFunction|UpdateScoreGaugeonServer))

(fn ConstructionScript)

(fn InitCamera
  (Class|HeadMountedDisplayFunctionLibrary|SetTrackingOrigin "Eye")
  (Transformation|SetRelativeLocation (Variables|Default|GetCamera) (Math|Vector|MakeVector 0.0 0.0 2e+01) false false)
  (Class|HeadMountedDisplayFunctionLibrary|ResetOrientationandPosition 0.0 "OrientationAndPosition"))

(fn InitCapture
  (params (Ref_Outer :type BP%20Tank%20Outer%20Object%20Reference))
  (if (Pawn|IsLocallyControlled)
    (Variables|/Script/Engine.SceneCaptureComponent2D|SetTextureTarget (Variables|/Game/Kawashima/BP/BP_Test/BP_Tank_Outer.BP_Tank_Outer_C|GetMain Ref_Outer) "/Game/Kawashima/Render_Main.Render_Main") ; メッシュのデフォルト値は空にしておくこと
  ))

(fn SetHPMaterial
  (params (HP_Now :type Float%20%28double-precision%29) (HP_Max :type Float%20%28double-precision%29))
  (Rendering|Material|SetScalarParameterValueonMaterials (Variables|Default|GetMesh_HP) "Value" (/ HP_Now HP_Max)))

(fn InitTimeText3D
  (bind _asbp_time_text_3d (Utilities|Casting|CastToBP_TimeText3D (Variables|/Script/Engine.ChildActorComponent|GetChildActor (Variables|Default|GetBP_TimeText3D))))
  (Variables|Default|SetRef_TimeText3D _asbp_time_text_3d))

(fn UpdateTimer
  (bind _ref_timetext3d (Variables|Default|GetRef_TimeText3D))
  (bind _asgs_domination (Utilities|Casting|CastToGS_Domination (Game|GetGameState)))
  (Utilities|IsValid _ref_timetext3d
    (:Is%20Valid
      (Default|SetTime _ref_timetext3d (Math|Float|Truncate (Variables|/Game/Iino/BP/GameState/GS_Domination.GS_Domination_C|GetTimeLimit _asgs_domination))) ; 秒での経過時間ないし残り時間を渡す
    )))

(fn TestBattleCountUp
  (return (+ (* (Math|Trig|Sin(Radians) (+ (Variables|Default|GetTestDelta) (Variables|Default|GetTestTime))) 5e+01) 5e+01)))

(fn SetShieldMaterial
  (params (CurrentShield :type Float%20%28double-precision%29) (MaxShield :type Float%20%28double-precision%29))
  (Rendering|Material|SetScalarParameterValueonMaterials (Variables|Default|GetMesh_Shield) "Value" (/ CurrentShield MaxShield)))

(fn UpdateScoreGauge
  (bind _asps_sphere_arena (Utilities|Casting|CastToPS_SphereArena (Variables|/Script/Engine.Pawn|GetPlayerState (Variables|Default|GetRef_Tank_Outer))))
  (bind _score (Default|GetPlayerScore _asps_sphere_arena))
  (Rendering|Material|SetScalarParameterValueonMaterials (Variables|Default|GetMesh_Table) "Value" (- 1e+02 (Math|Conversions|ToFloat(Integer) _score))))

(fn InitRaderTarget
  (bind _asgs_domination (Utilities|Casting|CastToGS_Domination (Game|GetGameState)))
  (bind _pawn (Default|GetOtherPlayerPawn _asgs_domination (Variables|Default|GetRef_Tank_Outer)))
  (Variables|Default|SetRaderTarget _pawn))