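; BP_Barrier is a barrier skill actor that animates its appearance when spawned.
; On BeginPlay it hides the frame mesh and starts a looping timer that steadily raises the "Dissolve" material parameter on the barrier mesh.
; As the value nears 1, it clears the timer and reveals the frame, using a threshold just below 1 to work around a suspected extra timer tick.
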(event Custom|カスタムイベント
  ;[1 1 1] 一定時間パラメータを渡すときに稼働させるイベント
  (bind _output_get (Variables|Default|SetTimer (+ (Variables|Default|GetTimer) 0.025)))
  (Rendering|Material|SetScalarParameterValueonMaterials (Variables|Default|GetMeshl_Barrier) "Dissolve" _output_get)
  (if (>= (Variables|Default|GetTimer) 0.9975)
    (Utilities|Time|ClearandInvalidateTimerbyHandle (Variables|Default|GetRef%20Handle))
    (Rendering|SetVisibility (Variables|Default|GetMesh_Barrier_Frame) true false)))

(event EventBeginPlay
  ;[1 1 1] 生成時に一定時間マテリアルパラメータを変動させるための処理
  (Rendering|SetVisibility (Variables|Default|GetMesh_Barrier_Frame) false false)
  (bind _returnvalue (Utilities|Time|SetTimerbyEvent (delegate Custom|カスタムイベント) 0.025 true))
  (Variables|Default|SetRef%20Handle _returnvalue))

(fn ConstructionScript)