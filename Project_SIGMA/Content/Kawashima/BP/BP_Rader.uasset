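; BP_Rader is a radar display that reflects the position and heading of an origin actor passed in by its caller.
; Init_Rader stores the origin's starting yaw in the Base material's RotateAdJust parameter.
; Update_Rader counter-rotates the Direction component and feeds location and normalized yaw into Base's material parameters.
; An author note reports slight stutter from per-frame material updates and proposes interval scanning instead.
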(event Custom|Init_Rader
  (params (Orizin :type Actor%20Object%20Reference))
  ;[1 1 1] アクタの向きをパラメータに割り当てて初期化
  (Rendering|Material|SetScalarParameterValueonMaterials (Variables|Default|GetBase) "RotateAdJust" (.yaw (Transformation|GetActorRotation Orizin))))

(event Custom|Update_Rader
  (params (Orizin :type Actor%20Object%20Reference))
  (bind _returnvalue (Transformation|GetActorRotation Orizin))
  ;[1 1 1] 向きと位置を読み取ってマテリアルに反映する　毎フレームマテリアルが切り替わっているので少しマテリアルの描画がカクつく　対処法としては一定間隔でスキャンするレーダーのような仕様にすること
  (Transformation|SetRelativeRotation (Variables|Default|GetDirection) (Math|Rotator|MakeRotator 0.0 0.0 (* (.yaw _returnvalue) -1.0)) false false)
  (Rendering|Material|SetVectorParameterValueonMaterials (Variables|Default|GetBase) "Position" (Transformation|GetActorLocation Orizin))
  (Rendering|Material|SetScalarParameterValueonMaterials (Variables|Default|GetBase) "ZRotation" (/ (.yaw _returnvalue) 3.6e+02)))

(fn ConstructionScript)