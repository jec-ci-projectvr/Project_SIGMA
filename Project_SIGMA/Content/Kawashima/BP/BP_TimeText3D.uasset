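; BP_TimeText3D is a Blueprint that displays a time value as minutes and seconds in 3D text.
; SetTime takes a count of seconds, writes the quotient by 60 to Text3DMinute and the remainder to Text3DSecond, prepending a zero to seconds below ten.
; It has no logic in its events or construction script, so the text changes only when SetTime is called.
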(event EventBeginPlay)

(event Collision|EventActorBeginOverlap
  (params (OtherActor :type Actor%20Object%20Reference)))

(event EventTick
  (params (DeltaSeconds :type Float%20%28single-precision%29)))

(fn ConstructionScript)

(fn SetTime
  (params (Time%28Second%29 :type Integer))
  (bind _returnvalue (Math|Integer|%(Integer) Time%28Second%29 60))
  (Class|Text3DComponent|SetText (Variables|Default|GetText3D_Minute) (Utilities|Text|ToText(Integer) (/ Time%28Second%29 60))) ; 分単位文字列設定
  (if (< _returnvalue 10) ; 10以下な01のように隙間なく文字を埋めるための分岐
    (Class|Text3DComponent|SetText (Variables|Default|GetText3D_Second) (Utilities|Text|ToText(String) (Utilities|String|Append "0" (Utilities|String|ToString(Integer) _returnvalue)))) ; 秒単位文字列設定
    (else
      (Class|Text3DComponent|SetText (Variables|Default|GetText3D_Second) (Utilities|Text|ToText(Integer) _returnvalue)))))