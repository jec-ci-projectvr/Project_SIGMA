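; BP_Sphere1 is a Blueprint of helper functions for render-target setup, HP and shield recovery.
; InitTextureTarget assigns a texture target to the passed object only if its owning Pawn is locally controlled.
; IsHPMax reports whether current HP has reached the maximum.
; GetNextShieldRecoveryTime scales the current interval by a factor, clamped to a minimum, to set recovery pacing.
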(fn ConstructionScript)

(fn InitTextureTarget
  (params (self2 :type Scene%20Capture%20Component%202D%20Object%20Reference) (NewParam :type Texture%20Render%20Target%202D%20Object%20Reference))
  (bind _aspawn (Utilities|Casting|CastToPawn (Components|GetOwner self2)))
  (if (Pawn|IsLocallyControlled _aspawn)
    (Variables|/Script/Engine.SceneCaptureComponent2D|SetTextureTarget self2 NewParam)))

(fn IsHPMax
  (return (>= (Variables|Default|GetHPNow) (Variables|Default|GetHPMax))))

(fn GetNextShieldRecoveryTime
  (params (CurrentInterval :type Float%20%28double-precision%29))
  (return (Math|Float|Max(Float) (* CurrentInterval (LocalVariables|Getfactor)) (LocalVariables|GetminimumInterval))))