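; BP_Sphere is a player-controlled pawn that moves, looks around and fires projectiles from left and right shoot points.
; BeginPlay sets stats, a floor tracking origin, camera position and pitch limits; axis inputs drive control-rotation-relative movement and look.
; Each fire input spawns a BP_Shot with local forward velocity, then calls CallHPChange as a test.
; Capsule overlaps with BP_Shot subtract HP, destroy the shot and trigger PlayerDead, which only prints a message.
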(event OnComponentBeginOverlap(CapsuleComponent)
  (params (OverlappedComponent :type Primitive%20Component%20Object%20Reference) (OtherActor :type Actor%20Object%20Reference) (OtherComp :type Primitive%20Component%20Object%20Reference) (OtherBodyIndex :type Integer) (bFromSweep :type Boolean) (SweepResult :type Hit%20Result%20Structure%20%28by%20ref%29))
  ;[1 1 1] 当たり判定とHPの増減
  (Development|PrintString "Hit") ; ヒットしたかどうか
  (bind _asbp_shot (Utilities|Casting|CastToBP_Shot OtherActor))
  (Development|PrintString "Hit is Shot") ; ヒットしたのが弾かどうか
  (Development|PrintString (Utilities|String|ToString(Integer) (Variables|Default|GetHP))) ; 引く前のＨPを出力
  (bind _output_get (Variables|Default|SetHP (- (Variables|Default|GetHP) (Variables|/Game/Kawashima/BP/BP_Shot.BP_Shot_C|GetDamage _asbp_shot))))
  (Actor|DestroyActor _asbp_shot)
  (Development|PrintString (Utilities|String|ToString(Integer) _output_get)) ; 引いたＨＰを出力
  (if (not (> _output_get 0))
    (CallFunction|PlayerDead)))

(event Custom|PlayerDead
  (Development|PrintString "アナタは死にました"))

(event EventBeginPlay
  (bind _returnvalue (Game|GetPlayerCameraManager 0))
  ;[1 1 1] 変数初期化
  (Variables|Default|SetHP 10)
  (Variables|Default|SetLookSens 1.0)
  (Variables|Default|SetMovePow 5.0)
  (Variables|Default|SetShotPow 3e+03)
  ;[1 1 1] 視点カメラ初期化
  (Class|HeadMountedDisplayFunctionLibrary|SetTrackingOrigin "Floor")
  (Transformation|SetRelativeLocation (Variables|Default|GetCamera) (Math|Vector|MakeVector 0.0 0.0 3e+01) false false)
  ;[1 1 1] 視野角制限：上下
  (Variables|/Script/Engine.PlayerCameraManager|SetViewPitchMax _returnvalue 45.0)
  (Variables|/Script/Engine.PlayerCameraManager|SetViewPitchMin _returnvalue -45.0))

(event Collision|EventActorBeginOverlap
  (params (OtherActor :type Actor%20Object%20Reference)))

(event EventTick
  (params (DeltaSeconds :type Float%20%28single-precision%29)))

(event Input|ActionEvents|InputActionFireLeft
  (params (Key :type Key%20Structure :default "None"))
  ;[1 1 1] 射撃：右
  (:Pressed
    (bind _returnvalue (Game|SpawnActorfromClass "/Game/Kawashima/BP/BP_Shot.BP_Shot_C" (Transformation|GetWorldTransform (Variables|Default|GetshootLeft)) "Undefined" "MultiplyWithRoot" 0 0))
    (Game|Components|ProjectileMovement|SetVelocityinLocalSpace (Variables|/Game/Kawashima/BP/BP_Shot.BP_Shot_C|GetProjectileMovement _returnvalue) (* (Math|Vector|MakeVector 1.0 0.0 0.0) (Variables|Default|GetShotPow)))
    ;[1 1 1] テスト
    (Default|CallHPChange)))

(event Input|ActionEvents|InputActionFireRight
  (params (Key :type Key%20Structure :default "None"))
  ;[1 1 1] 射撃：左
  (:Pressed
    (bind _returnvalue (Game|SpawnActorfromClass "/Game/Kawashima/BP/BP_Shot.BP_Shot_C" (Transformation|GetWorldTransform (Variables|Default|GetshootRight)) "Undefined" "MultiplyWithRoot" 0 0))
    (Game|Components|ProjectileMovement|SetVelocityinLocalSpace (Variables|/Game/Kawashima/BP/BP_Shot.BP_Shot_C|GetProjectileMovement _returnvalue) (* (Math|Vector|MakeVector 1.0 0.0 0.0) (Variables|Default|GetShotPow)))
    ;[1 1 1] テスト
    (Default|CallHPChange)))

(event Input|AxisEvents|InputAxisTurnRight/LeftMouse
  (params (AxisValue :type Float%20%28single-precision%29))
  ;[1 1 1] 視点入力：左右
  (Pawn|Input|AddControllerYawInput (* AxisValue (Variables|Default|GetLookSens))))

(event Input|AxisEvents|InputAxisLookUp/DownMouse
  (params (AxisValue :type Float%20%28single-precision%29))
  ;[1 1 1] 視点入力：上下
  (Pawn|Input|AddControllerPitchInput (* AxisValue (Variables|Default|GetLookSens))))

(event Input|AxisEvents|InputAxisMoveFor/Backward
  (params (AxisValue :type Float%20%28single-precision%29))
  ;[1 1 1] 移動入力：前後
  (Pawn|Input|AddMovementInput (Math|Vector|GetForwardVector (Pawn|GetControlRotation :!class /Script/Engine.Pawn)) (* AxisValue (Variables|Default|GetMovePow)) false))

(event Input|AxisEvents|InputAxisMoveRight/Left
  (params (AxisValue :type Float%20%28single-precision%29))
  ;[1 1 1] 移動入力：左右
  (Pawn|Input|AddMovementInput (Math|Vector|GetRightVector (Pawn|GetControlRotation :!class /Script/Engine.Pawn)) (* AxisValue (Variables|Default|GetMovePow)) false))

(fn ConstructionScript)