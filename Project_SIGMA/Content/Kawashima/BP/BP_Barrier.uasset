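; BP_Barrier is a barrier actor that plays a dissolve effect on its mesh when it spawns.
; BeginPlay starts a looping 0.05-second timer that accumulates a Timer value and feeds it to the Dissolve material parameter on MeshBarrier.
; Near full value, the timer clears itself one step early and makes MeshFrame visible.
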(event Custom|カスタムイベント
  ;[1 1 1] 一定時間パラメータを渡すときに稼働させるイベント
  (bind _output_get (Variables|Default|SetTimer (+ (Variables|Default|GetTimer) 0.05)))
  (Rendering|Material|SetScalarParameterValueonMaterials (Variables|Default|GetMesh_Barrier) "Dissolve" _output_get)
  (if (>= (Variables|Default|GetTimer) 0.95)
    (Utilities|Time|ClearandInvalidateTimerbyHandle (Variables|Default|GetRef%20Handle))
    (Rendering|SetVisibility (Variables|Default|GetMesh_Frame) true false)))

(event EventBeginPlay
  ;[1 1 1] 生成時に一定時間マテリアルパラメータを変動させるための処理
  (bind _returnvalue (Utilities|Time|SetTimerbyEvent (delegate Custom|カスタムイベント) 0.05 true))
  (Variables|Default|SetRef%20Handle _returnvalue))

(fn ConstructionScript)