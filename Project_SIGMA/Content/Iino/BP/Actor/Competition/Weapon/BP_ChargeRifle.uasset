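; Charge rifle weapon for the competition mode that builds charge through Shot calls and fires on StopShot.
; Each Charge call increments a counter while firing is allowed, playing owning-client sounds at the minimum and full charge thresholds.
; Fire resets the counter and calls the parent Fire only above the minimum, scaling damage with charge.
; Bullet size and speed use two tiers, boosted at full charge.
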(event Custom|PlayChargeSound_OwningClient
  (params (Sound :type Sound%20Base%20Object%20Reference) (Location :type Vector))
  (Audio|PlaySoundatLocation Sound Location "0, 0, 0" 1.0 1.0 0.0 0 0 0 0))

(event EventStopShot
  (CallFunction|Fire "0, 0, 0"))

(event EventShot
  (params (shotVelocity :type Vector :default "0, 0, 0"))
  (CallFunction|Charge))

(fn ConstructionScript
  (|CallParentFunction))

(fn Fire
  (params (ShotVelocity :type Vector :default "0, 0, 0"))
  (if (> (Variables|Default|GetChargeCount) (Variables|Default|GetMinChargeRequired))
    (if (== (Variables|Default|GetChargeCount) (Variables|Default|GetMaxCharge))
      (Variables|Default|SetBulletScale 3.0)
      (Variables|Default|SetBulletSpeed 5e+03)
      (else
        (Variables|Default|SetBulletScale 1.5)
        (Variables|Default|SetBulletSpeed 1.5e+03)))
    (Variables|Default|SetWeaponDamage (Math|Float|Truncate (Math|Float|MapRangeClamped (Variables|Default|GetChargeCount) (Variables|Default|GetMinChargeRequired) (Variables|Default|GetMaxCharge) 3.0 12.0)))
    (Variables|Default|SetChargeCount 0.0)
    (|CallParentFunction ShotVelocity)
    (else
      (Variables|Default|SetChargeCount 0.0))))

(fn SetCanShot
  (|CallParentFunction))

(fn Charge
  (bind _chargecount (Variables|Default|GetChargeCount))
  (bind _firingposition (Variables|Default|GetFiringPosition))
  (bind _returnvalue (Transformation|GetWorldTransform _firingposition))
  (bind _location (Math|Transform|BreakTransform _returnvalue))
  (if (Variables|Default|GetCanFire)
    (if (< _chargecount (Variables|Default|GetMaxCharge))
      ;[1 1 1] 効果音の再生
      (bind _result (Math|Float|IncrementFloat _chargecount)
        (:%20%20
          (if (== _result (Variables|Default|GetMinChargeRequired))
            (CallFunction|PlayChargeSoundOwningClient "/Game/Iino/Sound/SoundCue/SECue/FirstCharge_ChargeRifle.FirstCharge_ChargeRifle" _location)
            (elif (== _result (Variables|Default|GetMaxCharge))
              (CallFunction|PlayChargeSoundOwningClient "/Game/Iino/Sound/SoundCue/SECue/FullCharge_ChargeRifle.FullCharge_ChargeRifle" _location))))))))