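; Base bullet actor for competition weapons that delivers damage on overlap and destroys itself on impact.
; Overlaps send damage and the owner as attacker through BPI_Damageable, then spawn an impact effect; capture areas get the effect without damage.
; Blocking hits spawn a separate hit effect before destroying the bullet.
; SetAppearance forwards a material and Niagara trail to a multicast event that applies them to the mesh and trail.
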(event OnComponentBeginOverlap(Collicion_Bullet)
  (params (OverlappedComponent :type Primitive%20Component%20Object%20Reference) (OtherActor :type Actor%20Object%20Reference) (OtherComp :type Primitive%20Component%20Object%20Reference) (OtherBodyIndex :type Integer) (bFromSweep :type Boolean) (SweepResult :type Hit%20Result%20Structure%20%28by%20ref%29))
  ;[1 1 1] 弾命中時の処理
  (if (Utilities|DoesObjectImplementInterface OtherActor "/Game/Iino/BP/Interface/BPI_Damageable.BPI_Damageable_C")
    (Class|BPIDamageable|TakeHit(Message) OtherActor (Variables|Default|GetDamage) (Components|GetOwner))
    (else
      (Utilities|Casting|CastToBP_CaptureArea OtherActor)))
  (Niagara|SpawnSystematLocation "/ShootingVFX/sA_ShootingVfxPack/FX/NiagaraSystems/NS_Impact_1.NS_Impact_1" (.Location (Collision|BreakHitResult SweepResult)))
  (Development|PrintString "Hit")
  (Actor|DestroyActor))

(event OnComponentHit(Collicion_Bullet)
  (params (HitComponent :type Primitive%20Component%20Object%20Reference) (OtherActor :type Actor%20Object%20Reference) (OtherComp :type Primitive%20Component%20Object%20Reference) (NormalImpulse :type Vector :default "0, 0, 0") (Hit :type Hit%20Result%20Structure%20%28by%20ref%29))
  (Niagara|SpawnSystematLocation (Variables|Default|GetHitEffect) (.Location (Collision|BreakHitResult Hit)))
  (Actor|DestroyActor))

(event Custom|SetAppearance
  (params (NewMaterial :type Material%20Instance%20Object%20Reference) (NiagaraTrail :type Niagara%20System%20Object%20Reference))
  (CallFunction|SetAppearanceMulticast NewMaterial NiagaraTrail))

(event Custom|SetAppearance_Multicast
  (params (NewMaterial :type Material%20Instance%20Object%20Reference) (NiagaraTrail :type Niagara%20System%20Object%20Reference))
  (Rendering|Material|SetMaterial (Variables|Default|GetMesh_Bullet) 0 NewMaterial)
  (Class|NiagaraComponent|SetAsset (Variables|Default|GetBulletTrail) NiagaraTrail true))

(event EventBeginPlay)

(event Collision|EventActorBeginOverlap
  (params (OtherActor :type Actor%20Object%20Reference)))

(event EventTick
  (params (DeltaSeconds :type Float%20%28single-precision%29)))

(fn ConstructionScript)