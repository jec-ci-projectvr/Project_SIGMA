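; BP_Rocket is a rocket projectile that deals area damage on its first contact.
; An overlap or hit on its collision component triggers HitEffectMulticast and HitRocketOnServer, with an AlreadyHit flag guarding against repeat impacts.
; The server handler runs a sphere overlap at the impact point, sends TakeHitMessage damage to actors implementing BPI_Damageable, then destroys the rocket after a short delay.
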(event OnComponentBeginOverlap(Collicion_Bullet)
  (params (OverlappedComponent :type Primitive%20Component%20Object%20Reference) (OtherActor :type Actor%20Object%20Reference) (OtherComp :type Primitive%20Component%20Object%20Reference) (OtherBodyIndex :type Integer) (bFromSweep :type Boolean) (SweepResult :type Hit%20Result%20Structure%20%28by%20ref%29))
  (bind _location (Collision|BreakHitResult SweepResult))
  (if (not (Variables|Default|GetAlreadyHit))
    (CallFunction|HitEffectMulticast _location)
    (CallFunction|HitRocketonServer _location)
    (Variables|Default|SetAlreadyHit true)))

(event OnComponentHit(Collicion_Bullet)
  (params (HitComponent :type Primitive%20Component%20Object%20Reference) (OtherActor :type Actor%20Object%20Reference) (OtherComp :type Primitive%20Component%20Object%20Reference) (NormalImpulse :type Vector :default "0, 0, 0") (Hit :type Hit%20Result%20Structure%20%28by%20ref%29))
  (bind _location (Collision|BreakHitResult Hit))
  (if (not (Variables|Default|GetAlreadyHit))
    (CallFunction|HitEffectMulticast _location)
    (CallFunction|HitRocketonServer _location)
    (Variables|Default|SetAlreadyHit true)))

(event Custom|HitRocketOnServer
  (params (Transform :type Vector))
  (Development|PrintString "hit")
  (bind _outactors (Collision|SphereOverlapActors Transform (Variables|Default|GetDamageRadius) (Variables|Default|GetObject%20Types) 0))
  (for _array_element _outactors
    (if (Utilities|DoesObjectImplementInterface _array_element "/Game/Iino/BP/Interface/BPI_Damageable.BPI_Damageable_C")
      (Class|BPIDamageable|TakeHit(Message) _array_element (Variables|Default|GetDamage))
      (Development|PrintString "send")))
  (Utilities|FlowControl|Delay 0.1)
  (Actor|DestroyActor))

(event EventBeginPlay
  (|CallParentFunction) ; This node is disabled and will not be called.\nDrag off pins to build functionality.
)

(event EventTick
  (params (DeltaSeconds :type Float%20%28single-precision%29))
  (|CallParentFunction DeltaSeconds) ; This node is disabled and will not be called.\nDrag off pins to build functionality.
)

(fn ConstructionScript
  (|CallParentFunction))