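; BP_WeaponBase is a weapon base actor that fires BP_Bullet projectiles when its Shot event is triggered.
; Fire spawns one or more bullets at the firing position, applying material, scale, damage and lifespan from weapon settings.
; Each bullet gets a random horizontal and vertical spread on its local velocity.
; A CanFire flag blocks further shots until a fire-rate timer resets it, or immediately when the rate is zero.
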(event EventShot
  (CallFunction|Fire))

(fn ConstructionScript)

(fn SetRefireTimer
  (bind _firerate (Variables|Default|GetFireRate))
  (if (not (Variables|Default|GetCanFire))
    (if (!= _firerate 0.0)
      (bind _returnvalue (Utilities|Time|SetTimerbyFunctionName 0 "SetCanShot" _firerate))
      (Variables|Default|SetShotTimer _returnvalue)
      (else
        (CallFunction|SetCanShot)))))

(fn Fire
  (bind _horizontalspreadangle (Variables|Default|GetHorizontalSpreadAngle))
  (bind _verticalspreadangle (Variables|Default|GetVerticalSpreadAngle))
  (if (Variables|Default|GetCanFire)
    (for _index (range 0 (- (Variables|Default|GetBulletsFiredSimultaneously) 1))
      (bind _returnvalue (Game|SpawnActorfromClass "/Game/Iino/BP/Actor/Competition/Weapon/Bullet/BP_Bullet.BP_Bullet_C" (Transformation|GetWorldTransform (Variables|Default|GetFiringPosition)) "Undefined" "MultiplyWithRoot" 0 0))
      (Default|SetMaterial _returnvalue (Variables|Default|GetBulletMatInstance))
      (Transformation|SetActorScale3D _returnvalue (* (Transformation|GetActorScale3D _returnvalue) (Variables|Default|GetBulletScale)))
      (Variables|/Game/Iino/BP/Actor/Competition/Weapon/Bullet/BP_Bullet.BP_Bullet_C|SetDamage _returnvalue (Variables|Default|GetWeaponDamage))
      (Actor|SetLifeSpan _returnvalue (Variables|Default|GetBulletLifeSpan))
      (Game|Components|ProjectileMovement|SetVelocityinLocalSpace (Variables|/Game/Iino/BP/Actor/Competition/Weapon/Bullet/BP_Bullet.BP_Bullet_C|GetProjectileMovement _returnvalue) (* (Math|Vector|MakeVector 1.0 (Math|Random|RandomFloatinRange (* _horizontalspreadangle -1.0) _horizontalspreadangle) (Math|Random|RandomFloatinRange (* _verticalspreadangle -1.0) _verticalspreadangle)) (Variables|Default|GetBulletSpeed))))
    (Variables|Default|SetCanFire false)
    (CallFunction|SetRefireTimer)))

(fn SetCanShot
  (Variables|Default|SetCanFire true))