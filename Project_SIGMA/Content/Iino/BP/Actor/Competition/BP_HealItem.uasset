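; BP_HealItem is a spinning competition pickup that heals a player's BP_Sphere on contact.
; Tick rotates the actor, and the sphere overlap casts to BP_Sphere and skips players already at max HP.
; Otherwise an RPC event prints a pickup message, calls the player's HealEvent with HealValue and destroys the item.
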(event OnComponentBeginOverlap(Sphere)
  (params (OverlappedComponent :type Primitive%20Component%20Object%20Reference) (OtherActor :type Actor%20Object%20Reference) (OtherComp :type Primitive%20Component%20Object%20Reference) (OtherBodyIndex :type Integer) (bFromSweep :type Boolean) (SweepResult :type Hit%20Result%20Structure%20%28by%20ref%29))
  (bind _asbp_sphere (Utilities|Casting|CastToBP_Sphere OtherActor))
  (bind _ishpmax (Default|IsHPMax _asbp_sphere))
  (if (not _ishpmax)
    (CallFunction|RPCGetItem _asbp_sphere)))

(event Custom|RPC_GetItem
  (params (TargetPlayer :type BP%20Sphere%20Object%20Reference))
  (Development|PrintString "アイテムを取得")
  (Default|HealEvent TargetPlayer (Variables|Default|GetHealValue))
  (Actor|DestroyActor))

(event EventBeginPlay)

(event Collision|EventActorBeginOverlap
  (params (OtherActor :type Actor%20Object%20Reference)))

(event EventTick
  (params (DeltaSeconds :type Float%20%28single-precision%29))
  (Class|Actor|AddActorWorldRotation "0.000000,1.000000,0.000000") ; 回転させる
)

(fn ConstructionScript)