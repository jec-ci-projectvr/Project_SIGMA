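; BP_ItemSpawner is a competition-mode actor that spawns a heal item and respawns it after it is gone.
; It spawns a BP_HealItem at its Arrow transform on BeginPlay, only with authority, and keeps a reference.
; A looping one-second timer counts up while that item is invalid and spawns a new one once SpawnTime is reached.
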(event Custom|SpawnItem
  ;[1 1 1] アイテムのスポーン
  (Networking|SwitchHasAuthority
    (:Authority
      (bind _returnvalue (Game|SpawnActorfromClass "/Game/Iino/BP/Actor/Competition/BP_HealItem.BP_HealItem_C" (Transformation|GetWorldTransform (Variables|Default|GetArrow)) "Undefined" "MultiplyWithRoot" 0 0))
      (Variables|Default|SetSpawnedItem _returnvalue))))

(event Custom|AddDeltaTime
  (if (not (Utilities|IsValid (Variables|Default|GetSpawnedItem)))
    (bind _result (Math|Float|IncrementFloat (Variables|Default|GetDeltaTime))
      (:%20%20
        (bind _output_get (Variables|Default|SetDeltaTime _result))
        (if (>= _output_get (Variables|Default|GetSpawnTime))
          (CallFunction|SpawnItem)
          (Variables|Default|SetDeltaTime 0.0))))))

(event EventBeginPlay
  (CallFunction|SpawnItem)
  (Utilities|Time|SetTimerbyEvent (delegate Custom|AddDeltaTime) 1.0 true))

(event Collision|EventActorBeginOverlap
  (params (OtherActor :type Actor%20Object%20Reference)))

(event EventTick
  (params (DeltaSeconds :type Float%20%28single-precision%29)))

(fn ConstructionScript)