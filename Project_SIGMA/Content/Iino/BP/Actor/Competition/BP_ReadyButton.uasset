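; BP_ReadyButton is a hittable ready-up button for competition modes.
; When hit while not yet ready, it calls PlayerReady on the BP_Domination game mode, falling back to GM_Shootout, and sets IsReady so later hits are ignored.
; An RPC then swaps materials on its Sphere and Target meshes to show the ready state.
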(event Custom|Ready
  (bind _returnvalue (Game|GetGameMode))
  (bind _asbp_domination (Utilities|Casting|CastToBP_Domination _returnvalue)
    (:then
      (Default|PlayerReady _asbp_domination))
    (:CastFailed
      (bind _asgm_shootout (Utilities|Casting|CastToGM_Shootout _returnvalue))
      (Development|PrintString "Ready")
      (Default|PlayerReady _asgm_shootout)))
  (Variables|Default|SetIsReady true)
  (CallFunction|RPCReady))

(event Custom|RPC_Ready
  (Rendering|Material|SetMaterial (Variables|Default|GetSphere) 0 "/Game/Iino/Material/M_readyButton.M_readyButton")
  (Rendering|Material|SetMaterial (Variables|Default|GetTarget) 1 "/Game/Iino/Material/M_readyButton.M_readyButton"))

(event EventTakeHit
  (params (Damage :type Integer) (Attacker :type Actor%20Object%20Reference))
  (if (not (Variables|Default|GetIsReady))
    (CallFunction|Ready)))

(fn ConstructionScript)