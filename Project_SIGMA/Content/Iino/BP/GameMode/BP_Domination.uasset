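; BP_Domination runs the Domination mode's area rotation, keeping one randomly chosen BP_CaptureArea active at a time.
; On BeginPlay it gathers all capture areas and activates one after a short delay, while a looping timer calls ActivateNextArea.
; Each switch deactivates the current area and temporarily removes it from the array to avoid an immediate repeat.
; The initial pick rolls separately for activation and storage, so the stored area can differ from the active one.
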(event Custom|ActivateNextArea
  (bind _captureareas (Variables|Default|GetCaptureAreas))
  ;[1 1 1] TimerEvent_エリアの切り替え
  (Development|PrintString "エリア切り替え")
  (bind _output_get (Variables|Default|SetLastActivateArea (Variables|Default|GetCurretActivateArea)))
  (Default|AreaDeactivate _output_get)
  (bind _returnvalue (Utilities|Array|RemoveItem (Variables|Default|GetCaptureAreas) (Variables|Default|GetLastActivateArea)))
  (if _returnvalue
    (bind _output_get_2 (Variables|Default|SetCurretActivateArea (Utilities|Array|Get(acopy) _captureareas (Math|Random|RandomInteger (Utilities|Array|Length _captureareas)))))
    (Default|AreaActivate _output_get_2)
    (Utilities|Array|Add (Variables|Default|GetCaptureAreas) (Variables|Default|GetLastActivateArea))
    (else
      (Development|PrintString "エリアのインデックス排除に失敗しました"))))

(event Custom|InitializeArea
  ;[1 1 1] 変数の初期化
  (bind _outactors (Actor|GetAllActorsOfClass "/Game/Iino/BP/Actor/Competition/BP_CaptureArea.BP_CaptureArea_C"))
  (Utilities|FlowControl|Delay 2.0)
  (bind _output_get (Variables|Default|SetCaptureAreas _outactors))
  (Default|AreaActivate (Utilities|Array|Get(acopy) _output_get (Math|Random|RandomInteger (Utilities|Array|Length _output_get))))
  (Variables|Default|SetCurretActivateArea (Utilities|Array|Get(acopy) _output_get (Math|Random|RandomInteger (Utilities|Array|Length _output_get)))))

(event EventBeginPlay
  (CallFunction|InitializeArea)
  (Utilities|Time|SetTimerbyFunctionName 0 "ActivateNextArea" 1e+01 true))

(fn ConstructionScript)