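; Game state Blueprint providing shared helpers for sound, spawning, teleporting and player lookup.
; A server-named sound event relays to a multicast-named event that plays the 2D sound.
; PlayerTeleport spawns BP_Teleportation with target, destination and dissolve/spawn effects.
; GetOtherPlayerPawn searches AllPlayerPawn for a pawn other than the caller's, while GetInnerSpawnPoint only increments a counter and returns an origin transform.
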(event Custom|PlaySound2DOnServer
  (params (Sound :type Sound%20Base%20Object%20Reference))
  (CallFunction|PlaySound2DMulticast Sound))

(event Custom|PlaySound2DMulticast
  (params (Sound :type Sound%20Base%20Object%20Reference))
  (Audio|PlaySound2D Sound 1.0 1.0 0.0 0 0))

(event EventBeginPlay)

(event EventTick
  (params (DeltaSeconds :type Float%20%28single-precision%29)))

(fn ConstructionScript)

(fn GetInnerSpawnPoint
  (Math|Integer|IncrementInt (Variables|Default|GetInner%20Spawn%20Count)
    (:%20%20
      (return (Math|Transform|MakeTransform "0, 0, 0")))))

(fn PlayerTeleport
  (params (TeleporterSpawnTransform :type Transform) (TeleportTransform :type Transform) (Target :type Actor%20Object%20Reference))
  (bind (_location _rotation) (Math|Transform|BreakTransform TeleportTransform))
  (Game|SpawnActorfromClass "/TeleportVFX/Teleportation_VFX/Blueprints/BP_Teleportation.BP_Teleportation_C" TeleporterSpawnTransform "Undefined" "MultiplyWithRoot" 0 Target _location true false _rotation "(R=0.000000,G=0.565187,B=0.963542,A=1.000000)" 5e+01 1.0 2e+02 1.5 1.0 "0.000000,0.000000,0.000000" "/TeleportVFX/Teleportation_VFX/Particles/P_TeleportDissolve_01.P_TeleportDissolve_01" "/TeleportVFX/Teleportation_VFX/Particles/P_TeleportSpawn_01.P_TeleportSpawn_01" 0))

(fn GetOtherPlayerPawn
  (params (MyPawn :type Pawn%20Object%20Reference))
  (for _array_element (Variables|Default|GetAllPlayerPawn)
    (if (!= _array_element MyPawn)
      (LocalVariables|SetReturnPawn _array_element)))
  (return (LocalVariables|GetReturnPawn)))