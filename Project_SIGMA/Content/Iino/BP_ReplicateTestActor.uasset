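; BP_ReplicateTestActor is a test actor for replication that displays a running counter.
; On Tick, only the authority calls UpdateTimer, which increments CntNum by one each frame.
; Every instance, authority or remote, then writes CntNum to CountTEXT each tick, showing the value it holds locally.
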(event Custom|UpdateTimer
  (if true
    (Variables|Default|SetCntNum (+ (Variables|Default|GetCntNum) 1))))

(event EventBeginPlay)

(event Collision|EventActorBeginOverlap
  (params (OtherActor :type Actor%20Object%20Reference)))

(event EventTick
  (params (DeltaSeconds :type Float%20%28single-precision%29))
  (Networking|SwitchHasAuthority
    (:Authority
      (CallFunction|UpdateTimer))
    (:Remote
      _))
  (Rendering|Components|TextRender|SetText (Variables|Default|GetCountTEXT) (Utilities|Text|ToText(Integer) (Variables|Default|GetCntNum))))

(fn ConstructionScript)