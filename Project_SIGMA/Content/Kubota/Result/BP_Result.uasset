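; BP_Result places player spheres at win or lose positions for the result stage.
; On BeginPlay it caches the transforms of the BP_WinPoint and BP_LosePoint actors and gathers every BP_Sphere.
; SetRT then reads each sphere's Result flag from its PS_SphereArena player state and moves it to the matching transform, so all winners share one point and all losers the other.
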(event Custom|SetRT
  (for _array_element (Variables|Default|Getsphere)
    (bind _asps_sphere_arena (Utilities|Casting|CastToPS_SphereArena (Variables|/Script/Engine.Pawn|GetPlayerState _array_element)))
    (if (== (Variables|/Game/Iino/BP/PlayerState/PS_SphereArena.PS_SphereArena_C|GetResult _asps_sphere_arena) true)
      (Transformation|SetActorTransform _array_element (Variables|Default|GetWinTransform))
      (else
        (Transformation|SetActorTransform _array_element (Variables|Default|GetLoseTransform))))))

(event EventBeginPlay
  ;[1 1 1] それぞれの出現位置のトランスフォームを取得
  (bind _returnvalue (Actor|GetActorOfClass "/Game/Kubota/Result/BP_WinPoint.BP_WinPoint_C"))
  (Variables|Default|SetWinTransform (Transformation|GetActorTransform _returnvalue))
  (bind _returnvalue_2 (Actor|GetActorOfClass "/Game/Kubota/Result/BP_LosePoint.BP_LosePoint_C"))
  (Variables|Default|SetLoseTransform (Transformation|GetActorTransform _returnvalue_2))
  (bind _outactors (Actor|GetAllActorsOfClass "/Game/Kawashima/BP/BP_Sphere.BP_Sphere_C"))
  (Variables|Default|Setsphere _outactors)
  (CallFunction|SetRT))

(event EventTick
  (params (DeltaSeconds :type Float%20%28single-precision%29)))

(fn ConstructionScript)