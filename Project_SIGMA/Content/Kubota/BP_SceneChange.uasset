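; Scene-switching Blueprint that cycles through the title, game and result levels when Z is pressed.
; BeginPlay matches the current level name to store the next level's index in GameInstance_Main.
; The LevelChange macro starts a non-blocking stream load on Z, while its Tick-driven path adds a fade-out widget, then opens the level or shows a text widget if loading is unfinished.
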(event EventTick
  (params (DeltaSeconds :type Float%20%28single-precision%29))
  (Development|PrintString (Utilities|String|ToString(Integer) (Variables|/Game/Kubota/GameInstance_Main.GameInstance_Main_C|GetLevelNmb (stale EventBeginPlay _asgame_instance_main))))
  (Utilities|LevelChange (Utilities|Array|Get(acopy) (Utilities|Array|MakeArray (Variables|Default|GetTitleLevel) (Variables|Default|GetGameLevel) (Variables|Default|GetResultLevel)) (Variables|/Game/Kubota/GameInstance_Main.GameInstance_Main_C|GetLevelNmb (stale EventBeginPlay _asgame_instance_main))))
  (if (< (+ (Variables|/Game/Kubota/GameInstance_Main.GameInstance_Main_C|GetLevelNmb (stale EventBeginPlay _asgame_instance_main)) 1) 3)
    (Variables|/Game/Kubota/GameInstance_Main.GameInstance_Main_C|SetLevelNmb (stale EventBeginPlay _asgame_instance_main) (+ (Variables|/Game/Kubota/GameInstance_Main.GameInstance_Main_C|GetLevelNmb (stale EventBeginPlay _asgame_instance_main)) 1))
    (else
      (Variables|/Game/Kubota/GameInstance_Main.GameInstance_Main_C|SetLevelNmb (stale EventBeginPlay _asgame_instance_main) 0))))

(event EventBeginPlay
  (bind _asgame_instance_main (Utilities|Casting|CastToGameInstance_Main (Game|GetGameInstance)))
  (Utilities|SearchLevel)
  (Variables|/Game/Kubota/GameInstance_Main.GameInstance_Main_C|SetLevelNmb _asgame_instance_main (Variables|Default|Getatai)))

(event Input|KeyboardEvents|Z
  (params (Key :type Key%20Structure :default "None"))
  (:Pressed
    (Utilities|LevelChange (Utilities|Array|Get(acopy) (Utilities|Array|MakeArray (Variables|Default|GetTitleLevel) (Variables|Default|GetGameLevel) (Variables|Default|GetResultLevel)) (Variables|/Game/Kubota/GameInstance_Main.GameInstance_Main_C|GetLevelNmb (stale EventBeginPlay _asgame_instance_main)))) ; enters at execute2
  ))

(fn ConstructionScript)