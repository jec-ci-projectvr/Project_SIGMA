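; BP_Fead is a helper Blueprint that puts screen fade and loading text overlays on screen.
; Three custom events, EventFeadOut, EventFeadIn and EventLoadingText, each create their matching UMG widget and add it to the viewport.
; Each event ends in a Delay with nothing after it, and the Blueprint never removes the widgets it creates.
; BeginPlay, Tick and overlap events are unused.
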(event Custom|EventLoadingText
  (bind _returnvalue (UserInterface|CreateWidget "/Game/Kubota/UMG_text.UMG_text_C"))
  (UserInterface|Viewport|AddtoViewport _returnvalue 0)
  (Utilities|FlowControl|Delay 2.0))

(event Custom|EventFeadOut
  (bind _returnvalue (UserInterface|CreateWidget "/Game/Kubota/UMG_FadeOut.UMG_FadeOut_C"))
  (UserInterface|Viewport|AddtoViewport _returnvalue 0)
  (Utilities|FlowControl|Delay 1.0))

(event Custom|EventFeadIn
  (bind _returnvalue (UserInterface|CreateWidget "/Game/Kubota/UMG_FadeIn.UMG_FadeIn_C"))
  (UserInterface|Viewport|AddtoViewport _returnvalue 0)
  (Utilities|FlowControl|Delay 1.0))

(event EventBeginPlay)

(event Collision|EventActorBeginOverlap
  (params (OtherActor :type Actor%20Object%20Reference)))

(event EventTick
  (params (DeltaSeconds :type Float%20%28single-precision%29)))

(fn ConstructionScript)