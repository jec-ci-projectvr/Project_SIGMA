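; BP_LevelChange handles switching to a named level with a fade-out and loading text.
; LevelChange raises a loading flag, stream-loads the level hidden and without blocking, then marks the load finished.
; While the flag is set, Tick calls the fade-out dispatcher every frame and, after a short delay, either opens the level by name or calls the loading-text dispatcher if loading is unfinished.
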(event Custom|LevelChange
  (params (Lname :type Name))
  (bind _output_get (Variables|Default|SetLoadState true))
  (Game|LoadStreamLevel(byName) Lname false)
  (bind _output_get_2 (Variables|Default|SetLoadEnd true)))

(event EventTick
  (params (DeltaSeconds :type Float%20%28single-precision%29))
  (if (stale Custom|LevelChange _output_get)
    (Default|CallCallFeadOut)
    (Utilities|FlowControl|Delay 1.0)
    (if (stale Custom|LevelChange _output_get_2)
      (Game|OpenLevel(byName) (stale Custom|LevelChange Lname))
      (else
        (Default|CallCallLoadingText)
        (Utilities|FlowControl|Delay 2.0)))))

(fn ConstructionScript)