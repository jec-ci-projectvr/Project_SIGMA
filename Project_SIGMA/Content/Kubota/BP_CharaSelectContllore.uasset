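; BP_CharaSelectContllore handles keyboard input for character selection, fading in when play begins.
; A and B each set a name, color and index for the choice.
; X copies that choice into GameInstance_Main, then requests a change to NextLevel.
; A separate UMG_FadeIn widget creation chain is left unconnected and never runs.
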(event EventBeginPlay
  (Default|CallEventFeadin)
  (Utilities|FlowControl|Delay 1.0))

(event Input|KeyboardEvents|B
  (params (Key :type Key%20Structure :default "None"))
  (:Pressed
    (Variables|Default|SetName "B")
    (Variables|Default|SetColor "Bule")
    (Variables|Default|SetNmb 1)))

(event Input|KeyboardEvents|A
  (params (Key :type Key%20Structure :default "None"))
  (:Pressed
    (Variables|Default|SetName "A")
    (Variables|Default|SetColor "Red")
    (Variables|Default|SetNmb 0)))

(event Input|KeyboardEvents|X
  (params (Key :type Key%20Structure :default "None"))
  (:Pressed
    (bind _asgame_instance_main (Utilities|Casting|CastToGameInstance_Main (Game|GetGameInstance)))
    (Variables|/Game/Kubota/GameInstance_Main.GameInstance_Main_C|SetSelectNmb _asgame_instance_main (Variables|Default|GetNmb))
    (Variables|/Game/Kubota/GameInstance_Main.GameInstance_Main_C|SetSelectName _asgame_instance_main (Variables|Default|GetName))
    (Variables|/Game/Kubota/GameInstance_Main.GameInstance_Main_C|SetSelectColor _asgame_instance_main (Variables|Default|GetColor))
    (Default|CallEventLevelChange (Variables|Default|GetNextLevel))))

(fn ConstructionScript)